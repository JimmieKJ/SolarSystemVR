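; BP_Earth is the Earth planet actor in a VR solar system, with a Moon mesh and a name sprite.
; While enabled, Tick orbits it around the Sun and rotates Earth and Moon, scaling speed steeply by the VR character's scroller value.
; It also passes the toggleable name sprite to a camera-facing helper.
; A timeline fades the opacity of both dynamic hover materials, created in the construction script, for highlighting.
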(event EventBeginPlay)

(event Collision|EventActorBeginOverlap
  (params (OtherActor :type Actor%20Object%20Reference)))

(event EventTick
  (params (DeltaSeconds :type Float%20%28single-precision%29))
  (Utilities|FlowControl|Sequence
    (:then_0
      (if (Variables|Default|GetNameSpriteVisiblity)
        (CallFunction|NameSplitetoCamera (Variables|Default|GetMesh_Earth) (Variables|Default|GetPaperSpriteName))))
    (:then_1
      (if (Variables|Default|GetcanPlayRound)
        (bind _asbp_vrcharacter (Utilities|Casting|CastToBP_VRCharacter (Game|GetPlayerCharacter 0)))
        (Variables|Default|SetdeltaSeconds (* (* DeltaSeconds (* (Math|Float|Square (Math|Float|Square (Variables|/Game/Actors_Blueprints/BP_VRCharacter.BP_VRCharacter_C|GetscrollerValuesExp _asbp_vrcharacter))) (* (Variables|/Game/Actors_Blueprints/BP_VRCharacter.BP_VRCharacter_C|GetscrollerValuesExp _asbp_vrcharacter) 365.0))) 1e+02))
        (Utilities|FlowControl|Sequence
          (:then_0
            (CallFunction|RotateActorAroundSun (* (Variables|Default|GetdeltaSeconds) -1.0) "0, 0, 0" "0, 0,1.000000" self))
          (:then_1
            (CallFunction|RotateMovement (* (Variables|Default|GetdeltaSeconds) -365.0) (Variables|Default|GetMesh_Earth) (Variables|Default|GetStaticMeshMoon))))))))

(event EventHightLightPlaneMat
  (bind _learp (Timeline|Timeline_0 PlayFromStart)
    (:Update
      (Rendering|Material|SetScalarParameterValue (Variables|Default|GetearthMatInstance) "Opacity" _learp :!class /Script/Engine.MaterialInstanceDynamic)
      (Rendering|Material|SetScalarParameterValue (Variables|Default|GetmoonMatInstance) "Opacity" _learp :!class /Script/Engine.MaterialInstanceDynamic))))

(event EventHideNameSprite
  (Variables|Default|SetNameSpriteVisiblity (not (Variables|Default|GetNameSpriteVisiblity)))
  (Rendering|ToggleVisibility (Variables|Default|GetPaperSpriteName) false))

(fn ConstructionScript
  (bind _returnvalue (Rendering|Material|CreateDynamicMaterialInstance (Variables|Default|GetMesh_Earth) 0 "/Game/Materials/M_Earth_Hover_Inst.M_Earth_Hover_Inst" :!class /Script/Engine.PrimitiveComponent))
  (Variables|Default|SetearthMatInstance _returnvalue)
  (bind _returnvalue_2 (Rendering|Material|CreateDynamicMaterialInstance (Variables|Default|GetStaticMeshMoon) 0 "/Game/Materials/M_Moon_Hover_Inst.M_Moon_Hover_Inst" :!class /Script/Engine.PrimitiveComponent))
  (Variables|Default|SetmoonMatInstance _returnvalue_2))

(fn GetWorldLocationOfPlane
  (return (Transformation|GetWorldLocation (Variables|Default|GetDefaultSceneRoot))))