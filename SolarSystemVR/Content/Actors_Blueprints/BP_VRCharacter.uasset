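; VR player character with a toggleable scene menu, laser pointing, teleport and speed-driven "brain control" movement.
; Tick flickers forward, left and right cue widgets at distinct frame-count rates while the menu shows, and applies externally set movement speeds.
; A right-hand trace triggers menu widgets, drags the time slider, highlights BP_PlanePar actors and eases the capsule toward them while trigger is held.
; Holding Teleport draws a left-hand parabola; release moves the capsule to the hit.
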(event Custom|BeginDrawLine
  (bind _motioncontroller_l (Variables|Default|GetMotionController_L))
  (bind _returnvalue (Transformation|GetWorldTransform _motioncontroller_l))
  (bind (_location _rotation) (Math|Transform|BreakTransform _returnvalue))
  (Utilities|FlowControl|Gate true) ; enters at Open
)

(event Custom|EndDrawLine
  (bind _motioncontroller_l (Variables|Default|GetMotionController_L))
  (bind _returnvalue (Transformation|GetWorldTransform _motioncontroller_l))
  (bind (_location _rotation) (Math|Transform|BreakTransform _returnvalue))
  (Utilities|FlowControl|Gate true) ; enters at Close
)

(event Collision|EventActorBeginOverlap
  (params (OtherActor :type Actor%20Object%20Reference)))

(event EventTick
  (params (DeltaSeconds :type Float%20%28single-precision%29))
  (bind (_outposition _outorientation) (Class|SteamVRFunctionLibrary|GetHandPositionandOrientation 0 "Left"))
  (bind (_outposition_2 _outorientation_2) (Class|SteamVRFunctionLibrary|GetHandPositionandOrientation 0 "Right"))
  (bind _motioncontroller_r (Variables|Default|GetMotionController_R))
  (bind _capsulecomponent (Variables|Collision|GetCapsuleComponent))
  (bind _motioncontroller_l (Variables|Default|GetMotionController_L))
  (bind _capsulecomponent_2 (Variables|Collision|GetCapsuleComponent))
  (bind _widget_timepoint (Variables|Default|GetWidget_TimePoint))
  (bind _returnvalue (Transformation|GetWorldTransform _motioncontroller_l))
  (bind _returnvalue_2 (Transformation|GetWorldLocation _motioncontroller_r))
  (bind _returnvalue_3 (Transformation|GetWorldRotation _motioncontroller_r))
  (bind _relativelocation (Variables|/Script/Engine.SceneComponent|GetRelativeLocation _widget_timepoint))
  (bind (_location _rotation) (Math|Transform|BreakTransform _returnvalue))
  (bind _returnvalue_4 (Math|Vector|GetForwardVector _returnvalue_3))
  (bind (_x _y _z) (Math|Vector|BreakVector _relativelocation))
  (Variables|Default|SetDeltaSecondsVal DeltaSeconds)
  (Utilities|FlowControl|Sequence
    (:then_0
      (if (Variables|Default|GetDoesMenuTurnOn)
        ;[1 1 1] set frequency of control pic
        (if (< (Variables|Default|Geti_ForwardCount) 15)
          (Variables|Default|Seti_ForwardCount (+ (Variables|Default|Geti_ForwardCount) 1))
          (Rendering|SetVisibility (Variables|Default|GetWidget_MoveForward) (<= (Variables|Default|Geti_ForwardCount) 8) false)
          (else
            (Variables|Default|Seti_ForwardCount 0)))
        (else
          (Rendering|SetVisibility (Variables|Default|GetWidget_MoveForward) false false))))
    (:then_1
      (if (Variables|Default|GetDoesMenuTurnOn)
        (if (< (Variables|Default|Geti_TurnLCount) 12)
          (Variables|Default|Seti_TurnLCount (+ (Variables|Default|Geti_TurnLCount) 1))
          (Rendering|SetVisibility (Variables|Default|GetWidget_TurnLeft) (<= (Variables|Default|Geti_TurnLCount) 6) false)
          (else
            (Variables|Default|Seti_TurnLCount 0)))
        (else
          (Rendering|SetVisibility (Variables|Default|GetWidget_TurnLeft) false false))))
    (:then_2
      (if (Variables|Default|GetDoesMenuTurnOn)
        (if (< (Variables|Default|Geti_TurnRCount) 9)
          (Variables|Default|Seti_TurnRCount (+ (Variables|Default|Geti_TurnRCount) 1))
          (Rendering|SetVisibility (Variables|Default|GetWidget_TurnRight) (<= (Variables|Default|Geti_TurnRCount) 5) false)
          (else
            (Variables|Default|Seti_TurnRCount 0)))
        (else
          (Rendering|SetVisibility (Variables|Default|GetWidget_TurnRight) false false))))
    (:then_3
      ;[1 1 1] set hand position and rotation with model
      (Transformation|SetRelativeLocationAndRotation (Variables|Default|GetMotionController_L) _outposition _outorientation false false)
      (Transformation|SetRelativeLocationAndRotation (Variables|Default|GetMotionController_R) _outposition_2 _outorientation_2 false false)
      ;[1 1 1] line trance by channel
      (bind _outhit (Collision|LineTraceByChannel (+ _returnvalue_2 (* _returnvalue_4 2.0)) (+ _returnvalue_2 (* _returnvalue_4 5e+06)) "TraceTypeQuery1" false 0 "ForOneFrame" false "(R=0.006593,G=1.000000,B=0.000000,A=1.000000)" "(R=1.000000,G=0.017204,B=0.000000,A=1.000000)"))
      (bind _aswidget_component (Utilities|Casting|CastToWidgetComponent (.HitComponent (Collision|BreakHitResult _outhit)))
        (:then
          (bind _aswidget_hand_l_ui (Utilities|Casting|CastToWidget_HandL_UI (UserInterface|GetUserWidgetObject _aswidget_component))
            (:then
              (Variables|Default|SetCanCallTriggerEvent true)
              (bind _output_get (Variables|Default|SetLineTranWidget _aswidget_hand_l_ui))
              (Utilities|Casting|CastToBP_Hand_L_TimePoint _output_get)
              (if (Variables|Default|GetmoveTimePoint)
                (Transformation|SetRelativeLocation _widget_timepoint (Math|Vector|MakeVector _x (Math|Float|Clamp(Float) (- _y (.Y (Math|Vector|BreakVector (- (.Location (Collision|BreakHitResult _outhit)) (Transformation|GetWorldLocation (Variables|Default|GetWidget_TimePoint)))))) -4e+01 3e+01) _z) false false)
                (Variables|Default|SetscrollerValuesExp (/ (- (.X (Math|Vector|BreakVector (Transformation|GetWorldLocation (Variables|Default|GetWidget_TimePoint)))) (.X (Math|Vector|BreakVector (Transformation|GetWorldLocation (Variables|Default|GetWidget_TimeBar))))) 3e+01))))
            (:CastFailed
              (Variables|Default|SetCanCallTriggerEvent false))))
        (:CastFailed
          (Variables|Default|SetCanCallTriggerEvent false)
          (bind _asbp_plane_par (Utilities|Casting|CastToBP_PlanePar (.HitActor (Collision|BreakHitResult _outhit))))
          (Utilities|FlowControl|Sequence
            (:then_0
              (Default|HightLightPlaneMat _asbp_plane_par))
            (:then_1
              (bind _planeworldlocation (Default|GetWorldLocationOfPlane _asbp_plane_par))
              (if (Variables|Default|GetmoveTimePoint)
                (Transformation|AddWorldOffset _capsulecomponent (* (- _planeworldlocation (Transformation|GetWorldLocation _capsulecomponent)) 0.001) false false)))))))
    (:then_4
      ;[1 1 1] brain control persen move
      (Transformation|AddLocalOffset _capsulecomponent_2 (* (Math|Vector|MakeVector (Variables|Default|GetMoveForwardSpeed) 0.0 (Variables|Default|GetUpwardSpeed)) (Variables|Default|GetDeltaSecondsVal)) false false)
      (Transformation|AddLocalRotation _capsulecomponent_2 (Math|Rotator|MakeRotator 0.0 0.0 (* (Variables|Default|GetMoveRightSpeed) (Variables|Default|GetDeltaSecondsVal))) false false))
    (:then_5
      (Utilities|FlowControl|Gate true
        (:Exit
          (bind (_hitbool _hit) (Default|DrawLineParabolaDetection (Variables|Default|GetLaserTool) _location (Math|Vector|GetForwardVector _rotation)))
          (if (Variables|Default|GetcanMove)
            (if _hitbool
              (Transformation|SetWorldLocation (Variables|Collision|GetCapsuleComponent) (Math|Vector|MakeVector (.X (Math|Vector|BreakVector (.ImpactPoint (Collision|BreakHitResult _hit)))) (.Y (Math|Vector|BreakVector (.ImpactPoint (Collision|BreakHitResult _hit)))) (+ (.Z (Math|Vector|BreakVector (+ (.ImpactPoint (Collision|BreakHitResult _hit)) (Math|Vector|ProjectVectorontoPlane (- (Transformation|GetWorldLocation (Variables|Collision|GetCapsuleComponent)) (Transformation|GetWorldLocation (Variables|Default|GetCamera))) "0, 0, 0")))) 1.8e+02)) false false))
            (Variables|Default|SetcanMove false)
            (CallFunction|EndDrawLine)))))))

(event Input|ActionEvents|InputActionTriggerMenuItem
  (params (Key :type Key%20Structure :default "AnyKey"))
  ;[1 1 1] excute menu function
  (:Pressed
    (Variables|Default|SetmoveTimePoint true)
    (if (Variables|Default|GetCanCallTriggerEvent)
      (Default|SetImageColor (Variables|Default|GetLineTranWidget))))
  (:Released
    (Variables|Default|SetmoveTimePoint false)))

(event Input|ActionEvents|InputActionTeleport
  (params (Key :type Key%20Structure :default "AnyKey"))
  (:Pressed
    (CallFunction|BeginDrawLine))
  (:Released
    (Variables|Default|SetcanMove true)))

(event Input|ActionEvents|InputActionTurnOnMenu
  (params (Key :type Key%20Structure :default "AnyKey"))
  ;[1 1 1] turn on menu
  (:Pressed
    (bind _output_get (Variables|Default|SetDoesMenuTurnOn (not (Variables|Default|GetDoesMenuTurnOn))))
    (for _array_element (Components|GetChildrenComponents (Variables|Default|GetSceneMenu) false)
      (Rendering|SetVisibility _array_element _output_get false))))

(fn ConstructionScript
  (for _array_element (Components|GetChildrenComponents (Variables|Default|GetSceneMenu) false)
    (Rendering|SetVisibility _array_element (Variables|Default|GetDoesMenuTurnOn) false)))

(fn SetWidgetDefalutColor
  (Appearance|SetColorandOpacity (UserInterface|GetUserWidgetObject (Variables|Default|GetWidget_Reset)) (Math|Color|MakeColor 1.0 1.0 1.0) :!class /Script/UMG.UserWidget)
  (Appearance|SetColorandOpacity (UserInterface|GetUserWidgetObject (Variables|Default|GetWidget_GravityField)) (Math|Color|MakeColor 1.0 1.0 1.0) :!class /Script/UMG.UserWidget)
  (Appearance|SetColorandOpacity (UserInterface|GetUserWidgetObject (Variables|Default|GetWidget_Stop)) (Math|Color|MakeColor 1.0 1.0 1.0) :!class /Script/UMG.UserWidget)
  (Appearance|SetColorandOpacity (UserInterface|GetUserWidgetObject (Variables|Default|GetWidget_Orbits)) (Math|Color|MakeColor 1.0 1.0 1.0) :!class /Script/UMG.UserWidget)
  (Appearance|SetColorandOpacity (UserInterface|GetUserWidgetObject (Variables|Default|GetWidget_Quit)) (Math|Color|MakeColor 1.0 1.0 1.0) :!class /Script/UMG.UserWidget)
  (Appearance|SetColorandOpacity (UserInterface|GetUserWidgetObject (Variables|Default|GetWidget_TimePoint)) (Math|Color|MakeColor 1.0 1.0 1.0) :!class /Script/UMG.UserWidget)
  (Appearance|SetColorandOpacity (UserInterface|GetUserWidgetObject (Variables|Default|GetWidget_Sound)) (Math|Color|MakeColor 1.0 1.0 1.0) :!class /Script/UMG.UserWidget)
  (Appearance|SetColorandOpacity (UserInterface|GetUserWidgetObject (Variables|Default|GetWidget_Text)) (Math|Color|MakeColor 1.0 1.0 1.0) :!class /Script/UMG.UserWidget)
  (Appearance|SetColorandOpacity (UserInterface|GetUserWidgetObject (Variables|Default|GetWidget_TurnAround)) (Math|Color|MakeColor 1.0 1.0 1.0) :!class /Script/UMG.UserWidget)
  (Appearance|SetColorandOpacity (UserInterface|GetUserWidgetObject (Variables|Default|GetWidget_TimeBar)) (Math|Color|MakeColor 1.0 1.0 1.0) :!class /Script/UMG.UserWidget))