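; Jupiter planet actor for a VR solar system, orbiting the sun, spinning on itself and showing a name label.
; Tick updates the name sprite relative to the camera and, when CanPlayRound is set, drives orbit and spin at Jupiter-specific rates, with time scaled steeply by the VR character's scroller value.
; Events toggle the label and play a timeline that animates opacity on a dynamic hover material created in the construction script.
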(event EventTick
  (params (DeltaSeconds :type Float%20%28single-precision%29))
  (Utilities|FlowControl|Sequence
    (:then_0
      (if (Variables|Default|GetplanNameVisiblity)
        (CallFunction|NameSplitetoCamera (Variables|Default|GetMesh_Jupter) (Variables|Default|GetPaperSpriteName))))
    (:then_1
      (if (Variables|Default|GetcanPlayRound)
        (bind _asbp_vrcharacter (Utilities|Casting|CastToBP_VRCharacter (Game|GetPlayerCharacter 0)))
        (Variables|Default|SetdeltaSeconds (* (* DeltaSeconds (* (Math|Float|Square (Math|Float|Square (Variables|/Game/Actors_Blueprints/BP_VRCharacter.BP_VRCharacter_C|GetscrollerValuesExp _asbp_vrcharacter))) (* (Variables|/Game/Actors_Blueprints/BP_VRCharacter.BP_VRCharacter_C|GetscrollerValuesExp _asbp_vrcharacter) 365.0))) 1e+02))
        (Utilities|FlowControl|Sequence
          (:then_0
            (CallFunction|RotateActorAroundSun (/ (* (Variables|Default|GetdeltaSeconds) -1.0) 11.9) "0, 0, 0" "0, 0,1.000000" self))
          (:then_1
            (CallFunction|RotateMovement (* (* (Variables|Default|GetdeltaSeconds) -365.0) 2.4) (Variables|Default|GetMesh_Jupter) (Variables|Default|GetPlane2))))))))

(event EventHightLightPlaneMat
  (bind _learp (Timeline|Timeline_0 PlayFromStart)
    (:Update
      (Rendering|Material|SetScalarParameterValue (Variables|Default|GetplaneMatInstance) "Opacity" _learp :!class /Script/Engine.MaterialInstanceDynamic))))

(event EventHideNameSprite
  (Variables|Default|SetplanNameVisiblity (not (Variables|Default|GetplanNameVisiblity)))
  (Rendering|ToggleVisibility (Variables|Default|GetPaperSpriteName) false))

(fn ConstructionScript
  (bind _returnvalue (Rendering|Material|CreateDynamicMaterialInstance (Variables|Default|GetMesh_Jupter) 0 "/Game/Materials/M_Jupter_Hover_Inst.M_Jupter_Hover_Inst" :!class /Script/Engine.PrimitiveComponent))
  (Variables|Default|SetplaneMatInstance _returnvalue))

(fn GetWorldLocationOfPlane
  (return (Transformation|GetWorldLocation (Variables|Default|GetDefaultSceneRoot))))