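; BP_PlanePar is a parent actor class providing shared motion and label helpers for what appear to be planets orbiting a sun.
; RotateActorAroundSun orbits an actor about a given point and axis, turning its rotation to match, while RotateMovement spins two components locally, the second at a scaled rate.
; NameSpliteToCamera turns a name sprite toward the BP_VRCharacter's mesh.
; Highlight, hide-name and world-location functions are empty stubs, and no events drive the helpers here.
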(event EventBeginPlay)

(event Collision|EventActorBeginOverlap
  (params (OtherActor :type Actor%20Object%20Reference)))

(event EventTick
  (params (DeltaSeconds :type Float%20%28single-precision%29)))

(fn ConstructionScript)

(fn HideNameSprite)

(fn HightLightPlaneMat)

(fn NameSplitetoCamera
  (params (plane :type Scene%20Component%20Object%20Reference) (nameSprite :type Scene%20Component%20Object%20Reference))
  (bind _asbp_vrcharacter (Utilities|Casting|CastToBP_VRCharacter (Game|GetPlayerCharacter 0)))
  (bind _output_get (Variables|Default|SetinfoSpriteRot (Math|Rotator|MakeRotfromZ (- (Transformation|GetWorldLocation (Variables|/Script/Engine.Character|GetMesh _asbp_vrcharacter)) (Transformation|GetWorldLocation plane)))))
  (Transformation|SetWorldRotation nameSprite (Math|Rotator|Lerp(Rotator) (Variables|Default|GetinfoSpriteRot) (Math|Rotator|MakeRotator (- (.Roll (Math|Rotator|BreakRotator _output_get)) 9e+01) (- (.Pitch (Math|Rotator|BreakRotator _output_get)) -1.8e+02) (.Yaw (Math|Rotator|BreakRotator _output_get))) 1.0) false false))

(fn RotateActorAroundSun
  (params (Angle%20Def :type Float%20%28single-precision%29) (RotateSunPointVec :type Vector) (RotateSunAxisVec :type Vector) (WhichActor :type Actor%20Object%20Reference))
  (Transformation|SetActorLocationAndRotation WhichActor (+ (Math|Vector|RotateVectorAroundAxis (- (Transformation|GetActorLocation WhichActor) RotateSunPointVec) Angle%20Def RotateSunAxisVec) RotateSunPointVec) (Math|Rotator|CombineRotators (Transformation|GetActorRotation WhichActor) (Math|Vector|RotatorfromAxisandAngle RotateSunAxisVec Angle%20Def))))

(fn RotateMovement
  (params (AngleDef :type Float%20%28single-precision%29) (PlaneActor :type Static%20Mesh%20Component%20Object%20Reference) (Plane2Actor :type Static%20Mesh%20Component%20Object%20Reference))
  (Transformation|AddLocalRotation PlaneActor (Math|Rotator|MakeRotator 0.0 0.0 AngleDef) false false)
  (Transformation|AddLocalRotation Plane2Actor (Math|Rotator|MakeRotator 0.0 0.0 (* (/ AngleDef 365.0) 27.0)) false false))

(fn GetWorldLocationOfPlane
  (return "0, 0, 0"))