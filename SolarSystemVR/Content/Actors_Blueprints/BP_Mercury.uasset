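; BP_Mercury is the Mercury planet actor in a solar system scene with a VR character.
; When enabled, Tick orbits it around the sun and spins it, scaling time by the fifth power of the VR character's scroller value.
; Tick also updates its name sprite (named MarsSprite) relative to the camera while visible.
; Events toggle that label and play a timeline fading the dynamic hover material's opacity for highlighting.
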(event EventTick
  (params (DeltaSeconds :type Float%20%28single-precision%29))
  (Utilities|FlowControl|Sequence
    (:then_0
      (if (Variables|Default|GetplaneNameVisiblity)
        (CallFunction|NameSplitetoCamera (Variables|Default|GetStatic_Mercury) (Variables|Default|GetMars_Sprite))))
    (:then_1
      (if (Variables|Default|GetcanPlayRound)
        (bind _asbp_vrcharacter (Utilities|Casting|CastToBP_VRCharacter (Game|GetPlayerCharacter 0)))
        (Variables|Default|SetdeltaSeconds (* (* DeltaSeconds (* (Math|Float|Square (Math|Float|Square (Variables|/Game/Actors_Blueprints/BP_VRCharacter.BP_VRCharacter_C|GetscrollerValuesExp _asbp_vrcharacter))) (* (Variables|/Game/Actors_Blueprints/BP_VRCharacter.BP_VRCharacter_C|GetscrollerValuesExp _asbp_vrcharacter) 365.0))) 1e+02))
        (Utilities|FlowControl|Sequence
          (:then_0
            (CallFunction|RotateActorAroundSun (* (* (Variables|Default|GetdeltaSeconds) -1.0) 4.2) "0, 0, 0" "0, 0,1.000000" self))
          (:then_1
            (CallFunction|RotateMovement (/ (* (Variables|Default|GetdeltaSeconds) -365.0) 59.0) (Variables|Default|GetStatic_Mercury) (Variables|Default|GetPlane2))))))))

(event EventHightLightPlaneMat
  (bind _learp (Timeline|Timeline_0 PlayFromStart)
    (:Update
      (Rendering|Material|SetScalarParameterValue (Variables|Default|GetplaneMatInstance) "Opacity" _learp :!class /Script/Engine.MaterialInstanceDynamic))))

(event EventHideNameSprite
  (Variables|Default|SetplaneNameVisiblity (not (Variables|Default|GetplaneNameVisiblity)))
  (Rendering|ToggleVisibility (Variables|Default|GetMars_Sprite) false))

(fn ConstructionScript
  (bind _returnvalue (Rendering|Material|CreateDynamicMaterialInstance (Variables|Default|GetStatic_Mercury) 0 "/Game/Materials/M_Mercury_Hover_Inst.M_Mercury_Hover_Inst" :!class /Script/Engine.PrimitiveComponent))
  (Variables|Default|SetplaneMatInstance _returnvalue))

(fn GetWorldLocationOfPlane
  (return (Transformation|GetWorldLocation (Variables|Default|GetDefaultSceneRoot))))