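; BP_VRControl turns a brain-control command into movement speeds for the player's BP_VRCharacter.
; Each Tick it reads a direction index and speed from BrainControlCommond, setting forward speed for one index and right speed for two identically handled others.
; Those branches write the right speed to both character speed properties, so forward speed never reaches it.
; Idle or unknown indices zero only the local speeds, leaving the character unchanged.
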(event EventBeginPlay)

(event EventTick
  (params (DeltaSeconds :type Float%20%28single-precision%29))
  (bind _braincontrolcommond (Variables|Default|GetbrainControlCommond))
  (Variables|Default|SetControlPicIndex (Utilities|Array|Get(acopy) _braincontrolcommond))
  (Variables|Default|SetMoveSpeed (Utilities|Array|Get(acopy) _braincontrolcommond 1))
  (switch int (Variables|Default|GetControlPicIndex)
    (:Default
      (Variables|Default|SetPawnMoveForwardSpeed 0 :!label _label)
      (Variables|Default|SetPawnMoveRightSpeed 0))
    (:0
      (goto _label))
    (:1
      (Variables|Default|SetPawnMoveRightSpeed 0)
      (Variables|Default|SetPawnMoveForwardSpeed (Variables|Default|GetMoveSpeed))
      (bind _asbp_vrcharacter (Utilities|Casting|CastToBP_VRCharacter (Game|GetPlayerCharacter 0) :!label _label_2))
      (Variables|/Game/Actors_Blueprints/BP_VRCharacter.BP_VRCharacter_C|SetMoveForwardSpeed _asbp_vrcharacter (Math|Conversions|ToFloat(Integer) (Variables|Default|GetPawnMoveRightSpeed)))
      (Variables|/Game/Actors_Blueprints/BP_VRCharacter.BP_VRCharacter_C|SetMoveRightSpeed _asbp_vrcharacter (Math|Conversions|ToFloat(Integer) (Variables|Default|GetPawnMoveRightSpeed))))
    (:2
      (Variables|Default|SetPawnMoveForwardSpeed 0)
      (Variables|Default|SetPawnMoveRightSpeed (Variables|Default|GetMoveSpeed))
      (goto _label_2))
    (:3
      (Variables|Default|SetPawnMoveForwardSpeed 0)
      (Variables|Default|SetPawnMoveRightSpeed (Variables|Default|GetMoveSpeed))
      (goto _label_2))))

(fn ConstructionScript)