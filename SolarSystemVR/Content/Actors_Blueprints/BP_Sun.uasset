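; BP_Sun is the Sun actor, with a hover highlight material and a toggleable name sprite.
; The construction script creates a dynamic hover material on the mesh, whose Opacity HightLightPlaneMat animates through a timeline.
; HideNameSprite toggles the label's visibility and flag, and while the flag is set, Tick calls NameSpliteToCamera with the mesh and sprite.
; The sprite component is named JupiterSpriteName despite belonging to the Sun.
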(event EventBeginPlay)

(event Collision|EventActorBeginOverlap
  (params (OtherActor :type Actor%20Object%20Reference)))

(event EventTick
  (params (DeltaSeconds :type Float%20%28single-precision%29))
  (if (Variables|Default|GetNameSpriteVisibilty)
    (CallFunction|NameSplitetoCamera (Variables|Default|GetStaticMesh) (Variables|Default|GetJupiter_SpriteName))))

(event EventHightLightPlaneMat
  (bind _learp (Timeline|Timeline_2 PlayFromStart)
    (:Update
      (Rendering|Material|SetScalarParameterValue (Variables|Default|GetSunMaterial) "Opacity" _learp :!class /Script/Engine.MaterialInstanceDynamic))))

(event EventHideNameSprite
  (Variables|Default|SetNameSpriteVisibilty (not (Variables|Default|GetNameSpriteVisibilty)))
  (Rendering|ToggleVisibility (Variables|Default|GetJupiter_SpriteName) false))

(fn ConstructionScript
  (bind _returnvalue (Rendering|Material|CreateDynamicMaterialInstance (Variables|Default|GetStaticMesh) 0 "/Game/Materials/M_Sun_Hover_Inst.M_Sun_Hover_Inst" :!class /Script/Engine.PrimitiveComponent))
  (Variables|Default|SetSunMaterial _returnvalue))