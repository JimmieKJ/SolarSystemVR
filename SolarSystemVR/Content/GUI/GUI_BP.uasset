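; 3D controls-guide actor that displays flight and weapon inputs as arrow or ring meshes with key and mouse labels.
; The construction script creates dynamic material instances, grouped into yaw, pitch, roll, vertical, horizontal, fire and missile.
; Start/Reverse events drive a timeline per group to fade Opacity in and out.
; Tick slowly yaws the spring arm and turns each label toward the player camera, using its relative location as the look-at origin.
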(event Custom|YawStart
  (bind _alpha (Timeline|Timeline_0 Play)
    (:Update
      (Rendering|Material|SetScalarParameterValue (Variables|Default|GetYawInst) "Opacity" _alpha :!class /Script/Engine.MaterialInstanceDynamic))))

(event Custom|YawReverse
  (bind _alpha (Timeline|Timeline_0 Reverse)
    (:Update
      (Rendering|Material|SetScalarParameterValue (Variables|Default|GetYawInst) "Opacity" _alpha :!class /Script/Engine.MaterialInstanceDynamic))))

(event Custom|PitchStart
  (bind _alpha (Timeline|Timeline_1 Play)
    (:Update
      (Rendering|Material|SetScalarParameterValue (Variables|Default|GetPitchInst) "Opacity" _alpha :!class /Script/Engine.MaterialInstanceDynamic))))

(event Custom|PitchReverse
  (bind _alpha (Timeline|Timeline_1 Reverse)
    (:Update
      (Rendering|Material|SetScalarParameterValue (Variables|Default|GetPitchInst) "Opacity" _alpha :!class /Script/Engine.MaterialInstanceDynamic))))

(event Custom|HorizonStart
  (bind _alpha (Timeline|Timeline_4 Play)
    (:Update
      (Rendering|Material|SetScalarParameterValue (Variables|Default|GetHorizontalInst) "Opacity" _alpha :!class /Script/Engine.MaterialInstanceDynamic))))

(event Custom|HorizonReverse
  (bind _alpha (Timeline|Timeline_4 Reverse)
    (:Update
      (Rendering|Material|SetScalarParameterValue (Variables|Default|GetHorizontalInst) "Opacity" _alpha :!class /Script/Engine.MaterialInstanceDynamic))))

(event Custom|FireStarter
  (bind _alpha (Timeline|Timeline_5 Play)
    (:Update
      (Rendering|Material|SetScalarParameterValue (Variables|Default|GetFireInst) "Opacity" _alpha :!class /Script/Engine.MaterialInstanceDynamic))))

(event Custom|FireReverse
  (bind _alpha (Timeline|Timeline_5 Reverse)
    (:Update
      (Rendering|Material|SetScalarParameterValue (Variables|Default|GetFireInst) "Opacity" _alpha :!class /Script/Engine.MaterialInstanceDynamic))))

(event Custom|MissileStarter
  (bind _alpha (Timeline|Timeline_6 Play)
    (:Update
      (Rendering|Material|SetScalarParameterValue (Variables|Default|GetRightMouseInst) "Opacity" _alpha :!class /Script/Engine.MaterialInstanceDynamic))))

(event Custom|MissileReverse
  (bind _alpha (Timeline|Timeline_6 Reverse)
    (:Update
      (Rendering|Material|SetScalarParameterValue (Variables|Default|GetRightMouseInst) "Opacity" _alpha :!class /Script/Engine.MaterialInstanceDynamic))))

(event Custom|RollStart
  (bind _alpha (Timeline|Timeline_2 Play)
    (:Update
      (Rendering|Material|SetScalarParameterValue (Variables|Default|GetRollInst) "Opacity" _alpha :!class /Script/Engine.MaterialInstanceDynamic))))

(event Custom|RollReverse
  (bind _alpha (Timeline|Timeline_2 Reverse)
    (:Update
      (Rendering|Material|SetScalarParameterValue (Variables|Default|GetRollInst) "Opacity" _alpha :!class /Script/Engine.MaterialInstanceDynamic))))

(event Custom|VerticalStart
  (bind _alpha (Timeline|Timeline_3 Play)
    (:Update
      (Rendering|Material|SetScalarParameterValue (Variables|Default|GetVerticalInst) "Opacity" _alpha :!class /Script/Engine.MaterialInstanceDynamic))))

(event Custom|VerticalReverse
  (bind _alpha (Timeline|Timeline_3 Reverse)
    (:Update
      (Rendering|Material|SetScalarParameterValue (Variables|Default|GetVerticalInst) "Opacity" _alpha :!class /Script/Engine.MaterialInstanceDynamic))))

(event EventTick
  (params (DeltaSeconds :type Float%20%28single-precision%29))
  (Utilities|FlowControl|Sequence
    (:then_0
      (Transformation|AddRelativeRotation (Variables|Default|GetSpringArm) (Math|Rotator|MakeRotator 0.0 0.0 (* 5.0 DeltaSeconds)) false false))
    (:then_1
      (CallFunction|LookatFunction (Variables|Default|GetY))
      (CallFunction|LookatFunction (Variables|Default|GetFire))
      (CallFunction|LookatFunction (Variables|Default|GetE))
      (CallFunction|LookatFunction (Variables|Default|GetQ))
      (CallFunction|LookatFunction (Variables|Default|GetW))
      (CallFunction|LookatFunction (Variables|Default|GetS))
      (CallFunction|LookatFunction (Variables|Default|GetA))
      (CallFunction|LookatFunction (Variables|Default|GetD))
      (CallFunction|LookatFunction (Variables|Default|GetX))
      (CallFunction|LookatFunction (Variables|Default|GetMissile)))))

(fn ConstructionScript
  ;[0.5544 1 0.4592] Dynamic Material Instances
  ;;[1 1 1] Yaw
  (bind _returnvalue (Rendering|Material|CreateDynamicMaterialInstance (Variables|Default|GetLaunchPad2_Yaw) 0 "/Game/GUI/TexturesAndStuff/ArrowsMat.ArrowsMat" :!class /Script/Engine.PrimitiveComponent))
  (Variables|Default|SetYawInst _returnvalue)
  (bind _returnvalue_2 (Rendering|Material|CreateDynamicMaterialInstance (Variables|Default|GetA) 0 "/Game/GUI/TexturesAndStuff/DefaultTextMaterialOpaque.DefaultTextMaterialOpaque" :!class /Script/Engine.PrimitiveComponent))
  (Variables|Default|SetAInst _returnvalue_2)
  (bind _returnvalue_3 (Rendering|Material|CreateDynamicMaterialInstance (Variables|Default|GetD) 0 "/Game/GUI/TexturesAndStuff/DefaultTextMaterialOpaque.DefaultTextMaterialOpaque" :!class /Script/Engine.PrimitiveComponent))
  (Variables|Default|SetDInst _returnvalue_3)
  ;;[1 1 1] Pitch
  (bind _returnvalue_4 (Rendering|Material|CreateDynamicMaterialInstance (Variables|Default|GetLaunchPad2_Pitch) 0 "/Game/GUI/TexturesAndStuff/ArrowsMat.ArrowsMat" :!class /Script/Engine.PrimitiveComponent))
  (Variables|Default|SetPitchInst _returnvalue_4)
  (bind _returnvalue_5 (Rendering|Material|CreateDynamicMaterialInstance (Variables|Default|GetY) 0 "/Game/GUI/TexturesAndStuff/DefaultTextMaterialOpaque.DefaultTextMaterialOpaque" :!class /Script/Engine.PrimitiveComponent))
  (Variables|Default|SetMouseYInst _returnvalue_5)
  ;;[1 1 1] Roll
  (bind _returnvalue_6 (Rendering|Material|CreateDynamicMaterialInstance (Variables|Default|GetLaunchPad2_Roll) 0 "/Game/GUI/TexturesAndStuff/ArrowsMat.ArrowsMat" :!class /Script/Engine.PrimitiveComponent))
  (Variables|Default|SetRollInst _returnvalue_6)
  (bind _returnvalue_7 (Rendering|Material|CreateDynamicMaterialInstance (Variables|Default|GetX) 0 "/Game/GUI/TexturesAndStuff/DefaultTextMaterialOpaque.DefaultTextMaterialOpaque" :!class /Script/Engine.PrimitiveComponent))
  (Variables|Default|SetMouseXInst _returnvalue_7)
  ;;[1 1 1] Vertical
  (bind _returnvalue_8 (Rendering|Material|CreateDynamicMaterialInstance (Variables|Default|GetLaunchPad2_Vertical) 0 "/Game/GUI/TexturesAndStuff/ArrowsMat.ArrowsMat" :!class /Script/Engine.PrimitiveComponent))
  (Variables|Default|SetVerticalInst _returnvalue_8)
  (bind _returnvalue_9 (Rendering|Material|CreateDynamicMaterialInstance (Variables|Default|GetE) 0 "/Game/GUI/TexturesAndStuff/DefaultTextMaterialOpaque.DefaultTextMaterialOpaque" :!class /Script/Engine.PrimitiveComponent))
  (Variables|Default|SetEInst _returnvalue_9)
  (bind _returnvalue_10 (Rendering|Material|CreateDynamicMaterialInstance (Variables|Default|GetQ) 0 "/Game/GUI/TexturesAndStuff/DefaultTextMaterialOpaque.DefaultTextMaterialOpaque" :!class /Script/Engine.PrimitiveComponent))
  (Variables|Default|SetQInst _returnvalue_10)
  ;;[1 1 1] Horizontal
  (bind _returnvalue_11 (Rendering|Material|CreateDynamicMaterialInstance (Variables|Default|GetLaunchPad2_Horizontal) 0 "/Game/GUI/TexturesAndStuff/ArrowsMat.ArrowsMat" :!class /Script/Engine.PrimitiveComponent))
  (Variables|Default|SetHorizontalInst _returnvalue_11)
  (bind _returnvalue_12 (Rendering|Material|CreateDynamicMaterialInstance (Variables|Default|GetW) 0 "/Game/GUI/TexturesAndStuff/DefaultTextMaterialOpaque.DefaultTextMaterialOpaque" :!class /Script/Engine.PrimitiveComponent))
  (Variables|Default|SetWInst _returnvalue_12)
  (bind _returnvalue_13 (Rendering|Material|CreateDynamicMaterialInstance (Variables|Default|GetS) 0 "/Game/GUI/TexturesAndStuff/DefaultTextMaterialOpaque.DefaultTextMaterialOpaque" :!class /Script/Engine.PrimitiveComponent))
  (Variables|Default|SetSInst _returnvalue_13)
  ;;[1 1 1] Fire
  (bind _returnvalue_14 (Rendering|Material|CreateDynamicMaterialInstance (Variables|Default|GetLaunchPad2_Fire) 0 "/Game/GUI/TexturesAndStuff/ArrowsMat.ArrowsMat" :!class /Script/Engine.PrimitiveComponent))
  (Variables|Default|SetFireInst _returnvalue_14)
  (bind _returnvalue_15 (Rendering|Material|CreateDynamicMaterialInstance (Variables|Default|GetFire) 0 "/Game/GUI/TexturesAndStuff/DefaultTextMaterialOpaque.DefaultTextMaterialOpaque" :!class /Script/Engine.PrimitiveComponent))
  (Variables|Default|SetLeftMouseInst _returnvalue_15)
  (bind _returnvalue_16 (Rendering|Material|CreateDynamicMaterialInstance (Variables|Default|GetLaunchPad2_Fire2) 0 "/Game/GUI/TexturesAndStuff/ArrowsMat.ArrowsMat" :!class /Script/Engine.PrimitiveComponent))
  (Variables|Default|SetFire2Inst _returnvalue_16)
  (bind _returnvalue_17 (Rendering|Material|CreateDynamicMaterialInstance (Variables|Default|GetMissileRightRing) 0 "/Game/GUI/TexturesAndStuff/ArrowsMat.ArrowsMat" :!class /Script/Engine.PrimitiveComponent))
  (Variables|Default|SetMissileRing1Inst _returnvalue_17)
  (bind _returnvalue_18 (Rendering|Material|CreateDynamicMaterialInstance (Variables|Default|GetMissileLeftRing) 0 "/Game/GUI/TexturesAndStuff/ArrowsMat.ArrowsMat" :!class /Script/Engine.PrimitiveComponent))
  (Variables|Default|SetMissile2RingInst _returnvalue_18)
  (bind _returnvalue_19 (Rendering|Material|CreateDynamicMaterialInstance (Variables|Default|GetMissile) 0 "/Game/GUI/TexturesAndStuff/DefaultTextMaterialOpaque.DefaultTextMaterialOpaque" :!class /Script/Engine.PrimitiveComponent))
  (Variables|Default|SetRightMouseInst _returnvalue_19))

(fn LookatFunction
  (params (self2 :type Scene%20Component%20Object%20Reference))
  (Transformation|SetWorldRotation self2 (Math|Rotator|FindLookatRotation (Variables|/Script/Engine.SceneComponent|GetRelativeLocation self2) (Camera|GetCameraLocation (Game|GetPlayerCameraManager 0))) false false)
  (return))