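; AI controller for ToasterBP that steers the craft toward the player or back to reactors, using distance checks every tick.
; Within a set distance band it faces the player and applies distance-scaled thrust, braking through physics velocity when its velocity opposes its facing.
; Otherwise it loops over every ReactorBP, turning and thrusting toward each, and zeroing velocity inside a holding band.
; A sphere trace is present but never runs.
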(event EventBeginPlay
  (bind _astoaster_bp (Utilities|Casting|CastToToasterBP (Pawn|GetControlledPawn)))
  (bind _output_get (Variables|Default|SetToasterVar _astoaster_bp)))

(event EventTick
  (params (DeltaSeconds :type Float%20%28single-precision%29))
  (bind _returnvalue (Transformation|GetVelocity))
  (bind _toastervar (Variables|Default|GetToasterVar))
  (bind _toastervar_2 (Variables|Default|GetToasterVar))
  (bind _returnvalue_2 (Transformation|GetVelocity _toastervar_2))
  (bind _returnvalue_3 (Transformation|GetActorForwardVector _toastervar_2))
  (bind _returnvalue_4 (Math|Vector|DotProduct _returnvalue_2 _returnvalue_3))
  (bind _returnvalue_5 (/ _returnvalue_4 3.0))
  (bind _returnvalue_6 (Math|Float|InRange(Float) _returnvalue_4 _returnvalue_5 _returnvalue_4))
  (Transformation|SetActorRelativeRotation (Variables|Default|GetToasterVar) (Math|Rotator|FindLookatRotation (Transformation|GetActorLocation (Variables|Default|GetToasterVar)) (Transformation|GetActorLocation (Game|Player|GetPlayerPawn 0))))
  (if (Math|Float|InRange(Float) (Transformation|GetDistanceTo (stale EventBeginPlay _output_get) (Game|Player|GetPlayerPawn 0)) 5e+02 5e+05) ; Close enough to attack.
    (if _returnvalue_6
      (Default|Forward (Variables|Default|GetToasterVar) (Math|Float|SelectFloat (Math|Float|MapRangeClamped (Transformation|GetDistanceTo (stale EventBeginPlay _output_get) (Game|Player|GetPlayerPawn 0)) 1e+04 5e+05 0.0 1.0) 0.0 _returnvalue_6))
      (else
        (Physics|SetPhysicsLinearVelocity (Variables|/Game/Blueprints/AIStuff/ToasterBP.ToasterBP_C|GetPlane%20mesh (Variables|Default|GetToasterVar)) (Math|Interpolation|VInterpTo _returnvalue (/ _returnvalue 3.0) (Utilities|Time|GetWorldDeltaSeconds) 1.0) false "None") ; Space handbreak if it is behind the player. :P
      ))
    (else
      ;[1 1 1] Head back to the reactor
      (bind _outactors (Actor|GetAllActorsOfClass "/Game/Blueprints_Gameplay/ReactorBP.ReactorBP_C"))
      (for _array_element _outactors
        (Transformation|SetActorRelativeRotation (Variables|Default|GetToasterVar) (Math|Rotator|FindLookatRotation (Transformation|GetActorLocation _toastervar) (Transformation|GetActorLocation _array_element)))
        (if (Math|Float|InRange(Float) (Transformation|GetDistanceTo _toastervar _array_element) 7e+04 8e+04)
          (Physics|SetPhysicsLinearVelocity (Variables|/Game/Blueprints/AIStuff/ToasterBP.ToasterBP_C|GetPlane%20mesh (Variables|Default|GetToasterVar)) "0, 0, 0" false "None")
          (else
            (Default|Forward (Variables|Default|GetToasterVar) (Math|Float|MapRangeClamped (Transformation|GetDistanceTo _toastervar _array_element) 8e+04 4e+05 0.0 1.0))))))))

(fn ConstructionScript)