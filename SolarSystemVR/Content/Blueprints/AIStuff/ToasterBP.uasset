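; Enemy Cylon "Toaster" ship that shoots at the player's Viper and explodes once damage reaches its limit.
; Flight uses server-authoritative physics thrusters, main ones centered on mass, with angular-velocity damping and an instant brake.
; A looping CylonAI timer launches its child-actor missile once by range and facing, and line-traces ahead to toggle twin-gun fire.
; Distance-based pursuit, thruster FX, gun lights and destructible breakup are left unwired.
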(event OnComponentHit(Planemesh)
  (params (HitComponent :type Primitive%20Component%20Object%20Reference) (OtherActor :type Actor%20Object%20Reference) (OtherComp :type Primitive%20Component%20Object%20Reference) (NormalImpulse :type Vector) (Hit :type Hit%20Result%20Structure%20%28by%20ref%29))
  ;[1 1 1] Damage
  (bind _output_get (Variables|Default|SetDamageTaken (+ (Variables|Default|GetDamageTaken) (Math|Float|Truncate (Math|Vector|VectorLength (/ NormalImpulse (Physics|GetMass (Variables|Default|GetPlane%20mesh))))))))
  (if (>= _output_get (+ (Variables|Default|GetDamageTaken) (Math|Float|Truncate (Math|Vector|VectorLength (/ NormalImpulse (Physics|GetMass (Variables|Default|GetPlane%20mesh)))))))
    (Actor|DestroyActor)))

(event Custom|Fire
  (bind _plane_mesh (Variables|Default|GetPlane%20mesh))
  ;[1 1 1] GUNS
  (if (Variables|Default|GetCanFire)
    (Game|SpawnActorfromClass "/Game/Blueprints/AIStuff/ToasterProjectile.ToasterProjectile_C" (Transformation|GetSocketTransform _plane_mesh "Gun_Left" "RTS_World") "AlwaysSpawn" 0 0)
    (Utilities|FlowControl|Delay 0.1)
    (Game|SpawnActorfromClass "/Game/Blueprints/AIStuff/ToasterProjectile.ToasterProjectile_C" (Transformation|GetSocketTransform _plane_mesh "Gun_Right" "RTS_World") "AlwaysSpawn" 0 0)))

(event Custom|BoostDown
  ;[1 1 1] Boost
  (Networking|SwitchHasAuthority
    (:Authority
      (Variables|/Script/Engine.PhysicsThrusterComponent|SetThrustStrength (Variables|Default|GetMainEngine) 0.0))))

(event Custom|Forward
  (params (Thrust :type Float%20%28single-precision%29))
  (bind _mainengine (Variables|Default|GetMainEngine))
  ;[1 1 1] Forward Thrust
  (Networking|SwitchHasAuthority
    (:Authority
      (Variables|/Script/Engine.PhysicsThrusterComponent|SetThrustStrength _mainengine (* Thrust 1e+07))
      (Utilities|FlowControl|DoOnce false) ; enters at Reset
    )))

(event Custom|Vertical
  (params (Thrust :type Float%20%28single-precision%29))
  ;[1 1 1] Vertical Movement
  (Networking|SwitchHasAuthority
    (:Authority
      (Variables|/Script/Engine.PhysicsThrusterComponent|SetThrustStrength (Variables|Default|GetBottomThruster) (* Thrust 5e+06))
      (Variables|Default|SetVerticalThrust (< Thrust 0.0))
      (Variables|Default|SetVerticalLimit (Math|Float|InRange(Float) Thrust -0.1 0.1)))))

(event Custom|CylonAI
  (bind _returnvalue (Transformation|GetActorLocation))
  (bind _missile (Variables|Default|GetMissile))
  (bind _childactor (Variables|/Script/Engine.ChildActorComponent|GetChildActor _missile))
  (bind _astoaster_missile (Utilities|Casting|CastToToasterMissile _childactor))
  (Utilities|FlowControl|Sequence
    (:then_0
      (if (Variables|Default|GetCanFireMissile)
        (if (> (Math|Vector|DotProduct (Transformation|GetActorForwardVector (Game|Player|GetPlayerPawn 0)) (Math|Vector|GetForwardVector (Variables|Default|GetPlane%20mesh))) 0.0)
          ;[1 1 1] Missile
          (if (<= (Variables|Default|GetDistancetoPlayer) 1.5e+05)
            (Utilities|FlowControl|DoOnce false
              (:Completed
                (Utilities|IsValid (Variables|Default|GetMissile)
                  (:Is%20Valid
                    (Components|Activation|Activate (Variables|/Game/Blueprints/AIStuff/ToasterMissile.ToasterMissile_C|GetProjectile _astoaster_missile) false)
                    (Components|Tick|SetComponentTickEnabled _missile true)
                    (Actor|Tick|SetActorTickEnabled _astoaster_missile true)
                    (Default|SelfDestructionCountdown _astoaster_missile)
                    (Class|SceneComponent|DetachfromParent (Variables|Default|GetMissile) true true)
                    (Utilities|FlowControl|Delay 1.0)
                    (Collision|SetCollisionProfileName (Variables|/Game/Blueprints/AIStuff/ToasterMissile.ToasterMissile_C|GetCollisionComponent _astoaster_missile) "PhysicsActor" :!class /Script/Engine.PrimitiveComponent)))))))))
    (:then_1
      (bind _outhit (Collision|LineTraceByChannel _returnvalue (+ _returnvalue (* (Math|Vector|GetForwardVector (Transformation|GetActorRotation)) 2e+05)) "TraceTypeQuery1" true 0 "None"))
      (if (.bblockinghit _outhit)
        (Utilities|Casting|CastToViperBP (.hitactor _outhit)
          (:then
            (Utilities|FlowControl|DoOnce false :!label _label
              (:Completed
                (CallFunction|FireCustom)
                (goto _label_2 Reset))))
          (:CastFailed
            (Utilities|FlowControl|DoOnce false :!label _label_2
              (:Completed
                (CallFunction|FireCustomEnd)
                (goto _label Reset)))))))))

(event Custom|TickEvents
  (params (ThrustRight :type Float%20%28single-precision%29) (ThrustLeft :type Float%20%28single-precision%29) (Roll :type Boolean) (Roll2 :type Boolean) (ThrustUp :type Float%20%28single-precision%29) (AngVelocity :type Vector) (NoseUp :type Boolean) (NoseUpLimit :type Boolean) (ResetVelocity :type Boolean))
  (Networking|SwitchHasAuthority
    (:Authority
      (Variables|Default|SetRoll2 Roll2)
      (Variables|Default|SetRoll Roll)
      (Variables|/Script/Engine.PhysicsThrusterComponent|SetThrustStrength (Variables|Default|GetRollThruster%20Left) ThrustLeft)
      (Variables|/Script/Engine.PhysicsThrusterComponent|SetThrustStrength (Variables|Default|GetRollThruster%20Right) ThrustRight)
      (Variables|Default|SetAngular%20Velocity AngVelocity)
      (Variables|/Script/Engine.PhysicsThrusterComponent|SetThrustStrength (Variables|Default|GetNoseUpDown) ThrustUp)
      (Variables|Default|SetNoseUp NoseUp)
      (Variables|Default|SetNoseUpLimit NoseUpLimit)
      (if ResetVelocity
        ;[1 1 1] Reset Angular Velocity - Counter thrust for mouse control to make it feel more "game friendly"
        (Utilities|FlowControl|DoOnce false :!label _label
          (:Completed
            (bind _newtrack_0 (Timeline|Angular_Reset PlayFromStart)
              (:Update
                (Class|PrimitiveComponent|SetPhysicsAngularVelocity (Variables|Default|GetPlane%20mesh) (Math|Vector|Lerp(Vector) (Variables|Default|GetAngular%20Velocity) (/ (Variables|Default|GetAngular%20Velocity) 1.3) _newtrack_0) false "None")))))
        (else
          (goto _label Reset))))))

(event Custom|FireCustom
  ;[1 1 1] GUNS
  (bind _returnvalue (Utilities|Time|SetTimerbyEvent (delegate Custom|Fire) 0.2 true)))

(event Custom|FireCustomEnd
  ;[1 1 1] GUNS
  (Utilities|Time|ClearandInvalidateTimerbyHandle (stale Custom|FireCustom _returnvalue)))

(event Custom|ZeroSpeed
  (params (Thrust :type Float%20%28single-precision%29))
  ;[1 1 1] Forward Thrust
  (Networking|SwitchHasAuthority
    (:Authority
      (Utilities|FlowControl|DoOnce false
        (:Completed
          (Variables|/Script/Engine.PhysicsThrusterComponent|SetThrustStrength (Variables|Default|GetMainEngine) 0.0))))))

(event Custom|Yaw
  (params (Thrust :type Float%20%28single-precision%29))
  ;[1 1 1] Yaw Thruster
  (Networking|SwitchHasAuthority
    (:Authority
      (Variables|/Script/Engine.PhysicsThrusterComponent|SetThrustStrength (Variables|Default|GetYawThruster) (* Thrust 6e+05 -1.0))
      (Variables|Default|SetYawLeft (< Thrust 0.0))
      (Variables|Default|SetYawRight (> Thrust 0.0)))))

(event Custom|InstantBreak
  ;[1 1 1] Insta Break - just an option if you start to feel sick and want to stop immediately!
  (Networking|SwitchHasAuthority
    (:Authority
      (Physics|SetPhysicsLinearVelocity "0, 0, 0" false "None")
      (Class|PrimitiveComponent|SetPhysicsAngularVelocity "0, 0, 0" false "None"))))

(event Custom|BoostUp
  ;[1 1 1] Boost
  (Networking|SwitchHasAuthority
    (:Authority
      (Variables|/Script/Engine.PhysicsThrusterComponent|SetThrustStrength (Variables|Default|GetMainEngine) 1e+08))))

(event EventTick
  (params (DeltaSeconds :type Float%20%28single-precision%29))
  (bind _returnvalue (Class|Actor|GetInputAxisKeyValue))
  (bind _returnvalue_2 (Class|Actor|GetInputAxisKeyValue))
  (bind _returnvalue_3 (* 2e+06 _returnvalue_2))
  (Variables|Default|SetDistancetoPlayer (Transformation|GetDistanceTo (Game|Player|GetPlayerPawn 0)))
  (Utilities|FlowControl|Sequence
    (:then_0
      (bind _returnvalue_4 (Class|PrimitiveComponent|GetPhysicsAngularVelocity "None"))
      (CallFunction|TickEvents _returnvalue_3 _returnvalue_3 (< _returnvalue_2 0.0) (> _returnvalue_2 0.0) (* 2e+06 _returnvalue) _returnvalue_4 (< _returnvalue 0.0) (Math|Float|InRange(Float) _returnvalue -0.2 0.2) (and (Math|Float|InRange(Float) _returnvalue_2 -0.1 0.1) (Math|Float|InRange(Float) _returnvalue -0.1 0.1))))))

(event EventBeginPlay
  (Utilities|Time|SetTimerbyEvent (delegate Custom|CylonAI) 0.01 true))

(event Game|Damage|EventAnyDamage
  (params (Damage :type Float%20%28single-precision%29) (DamageType :type Damage%20Type%20Object%20Reference) (InstigatedBy :type Controller%20Object%20Reference) (DamageCauser :type Actor%20Object%20Reference))
  ;[1 1 1] Damage
  (bind _output_get (Variables|Default|SetDamageTaken (+ (Variables|Default|GetDamageTaken) (Math|Float|Truncate Damage))))
  (if (>= _output_get (Variables|Default|GetMaxDamage))
    (bind _returnvalue (Effects|SpawnEmitteratLocation "/Game/Particles/EnemyDestroyed.EnemyDestroyed" (Transformation|GetActorLocation)))
    (Class|SceneComponent|DetachfromParent _returnvalue true true)
    (Actor|DestroyActor)))

(event Collision|EventHit
  (params (MyComp :type Primitive%20Component%20Object%20Reference) (Other :type Actor%20Object%20Reference) (OtherComp :type Primitive%20Component%20Object%20Reference) (bSelfMoved :type Boolean) (HitLocation :type Vector :default "0, 0, 0") (HitNormal :type Vector :default "0, 0, 0") (NormalImpulse :type Vector :default "0, 0, 0") (Hit :type Hit%20Result%20Structure%20%28by%20ref%29))
  ;[1 1 1] Kill speed when colliding
  (Variables|/Script/Engine.PhysicsThrusterComponent|SetThrustStrength (Variables|Default|GetMainEngine) 1e+03))

(event Input|ActionEvents|InputActionBreak
  (params (Key :type Key%20Structure :default "AnyKey"))
  ;[1 1 1] Insta Break - just an option if you start to feel sick and want to stop immediately!
  (:Pressed
    (CallFunction|InstantBreak)))

(fn ConstructionScript
  (bind _returnvalue (Rendering|Material|CreateDynamicMaterialInstance (Variables|Default|GetPlane%20mesh) 1 0 :!class /Script/Engine.PrimitiveComponent))
  (Variables|Default|SetSplingMatInst _returnvalue)
  (bind _returnvalue_2 (Physics|GetCenterOfMass (Variables|Default|GetPlane%20mesh) "None"))
  ;[1 1 1] Set the main thrusters(vertical and horizontal) locations exactly on CoM
  (Transformation|SetWorldLocation (Variables|Default|GetMainEngine) _returnvalue_2 false false)
  (Transformation|SetWorldLocation (Variables|Default|GetBottomThruster) _returnvalue_2 false false))