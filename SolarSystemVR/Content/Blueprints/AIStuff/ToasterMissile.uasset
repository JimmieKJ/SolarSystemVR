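; Homing missile projectile that chases the player's Viper plane and explodes with radial damage.
; SelfDestructionCountdown starts the trail and fire effects, sets the plane mesh as homing target, alerts the Viper and begins a 20-second fuse.
; Tick reports proximity to the Viper and eases rotation toward it.
; Timeout, hit, randomized close range or lost target all feed one DoOnce detonation, which also clears the alert.
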(event OnComponentHit(CollisionComponent)
  (params (OtherActor :type Actor%20Object%20Reference) (OtherComp :type Primitive%20Component%20Object%20Reference) (NormalImpulse :type Vector :default "0, 0, 0") (Hit :type Hit%20Result%20Structure%20%28by%20ref%29))
  (bind _returnvalue (Transformation|GetActorLocation))
  (Utilities|FlowControl|DoOnce false
    (:Completed
      (Class|GameplayStatics|ApplyRadialDamagewithFalloff 2.5e+03 5e+02 _returnvalue 5e+02 1e+04 1.0 "/Game/Blueprints/DamageType_Missile.DamageType_Missile_C" 0 self 0 "ECC_Visibility")
      (bind _returnvalue_2 (Effects|SpawnEmitteratLocation "/Game/Particles/P_MissileExplosion.P_MissileExplosion" _returnvalue))
      (Class|SceneComponent|DetachfromParent _returnvalue_2 false true)
      (Default|MissileDestroyed (Variables|Default|GetTarget)) ; Stop Alert in Viper
      (Actor|DestroyActor))))

(event OnComponentBeginOverlap(CollisionComponent)
  (params (OtherActor :type Actor%20Object%20Reference) (OtherComp :type Primitive%20Component%20Object%20Reference) (OtherBodyIndex :type Integer) (bFromSweep :type Boolean) (SweepResult :type Hit%20Result%20Structure%20%28by%20ref%29)))

(event Custom|SelfDestructionCountdown
  (bind _returnvalue (Game|Player|GetPlayerPawn 0))
  (bind _returnvalue_2 (Transformation|GetActorLocation))
  (bind _asviper_bp (Utilities|Casting|CastToViperBP _returnvalue))
  ;[1 1 1] Destroy after a while so that the projectile doesn't go into space and exist forever and ever and ever and ever...
  (Components|Activation|Activate (Variables|Default|GetMissileTrail) false)
  (if (Class|Actor|IsActorTickEnabled)
    (Components|Activation|Activate (Variables|Default|GetMissileFire) false)
    (Variables|Default|SetTarget _asviper_bp)
    (Variables|/Script/Engine.ProjectileMovementComponent|SetHomingTargetComponent (Variables|MyProjectile|GetProjectile) (Variables|/Game/Blueprints/ViperBP.ViperBP_C|GetPlane%20mesh (Variables|Default|GetTarget)))
    (Default|IncomingMissile _asviper_bp) ; Start Alert in Viper
    (Utilities|FlowControl|Delay 2e+01)
    (Utilities|FlowControl|DoOnce false
      (:Completed
        (Class|GameplayStatics|ApplyRadialDamagewithFalloff 2.5e+03 5e+02 _returnvalue_2 5e+02 1e+04 1.0 "/Game/Blueprints/DamageType_Missile.DamageType_Missile_C" 0 self 0 "ECC_Visibility")
        (bind _returnvalue_3 (Effects|SpawnEmitteratLocation "/Game/Particles/P_MissileExplosion.P_MissileExplosion" _returnvalue_2))
        (Class|SceneComponent|DetachfromParent _returnvalue_3 false true)
        (Default|MissileDestroyed (Variables|Default|GetTarget)) ; Stop Alert in Viper
        (Actor|DestroyActor)))))

(event EventBeginPlay
  ;[1 1 1] Destroy after a while so that the projectile doesn't go into space and exist forever and ever and ever and ever...
)

(event EventTick
  (params (DeltaSeconds :type Float%20%28single-precision%29))
  (bind _returnvalue (Transformation|GetActorLocation))
  (bind _target (Variables|Default|GetTarget))
  (if (Class|Actor|IsActorTickEnabled)
    (Utilities|IsValid _target
      (:Is%20Valid
        (Default|ProximityEvent _target (< (Transformation|GetDistanceTo (Variables|Default|GetTarget)) 4e+04))
        (Utilities|FlowControl|Sequence
          (:then_0
            (if (Math|Float|InRange(Float) (Transformation|GetDistanceTo (Variables|Default|GetTarget)) 0.0 (Math|Random|RandomFloatinRange 3e+02 7.5e+02))
              (Utilities|FlowControl|DoOnce false :!label _label
                (:Completed
                  (Class|GameplayStatics|ApplyRadialDamagewithFalloff 2.5e+03 5e+02 _returnvalue 5e+02 1e+04 1.0 "/Game/Blueprints/DamageType_Missile.DamageType_Missile_C" 0 self 0 "ECC_Visibility")
                  (bind _returnvalue_2 (Effects|SpawnEmitteratLocation "/Game/Particles/P_MissileExplosion.P_MissileExplosion" _returnvalue))
                  (Class|SceneComponent|DetachfromParent _returnvalue_2 false true)
                  (Default|MissileDestroyed (Variables|Default|GetTarget)) ; Stop Alert in Viper
                  (Actor|DestroyActor)))))
          (:then_1
            (Transformation|SetActorRotation (Math|Interpolation|RInterpTo (Transformation|GetActorRotation) (Math|Rotator|FindLookatRotation (Transformation|GetActorLocation) (Transformation|GetWorldLocation (Variables|/Game/Blueprints/ViperBP.ViperBP_C|GetPlane%20mesh (Variables|Default|GetTarget)))) (Utilities|Time|GetWorldDeltaSeconds) 0.5)))))
      (:Is%20Not%20Valid
        (goto _label)))))

(fn ConstructionScript)