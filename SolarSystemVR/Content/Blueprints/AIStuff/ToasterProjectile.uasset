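; Toaster enemy bullet projectile that launches with random spread and self-destroys on impact or after a short timeout.
; Hits deal randomized point damage, spawn an explosion and fire a radial impulse; the Toaster-tagged branch uses minimal damage with no damaged actor set.
; Metal surfaces also play an impact sound scaled by game-instance FX volume.
; The construction script tints the bullet blue through a dynamic material.
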(event OnComponentHit(CollisionComponent)
  (params (OtherActor :type Actor%20Object%20Reference) (OtherComp :type Primitive%20Component%20Object%20Reference) (NormalImpulse :type Vector) (Hit :type Hit%20Result%20Structure%20%28by%20ref%29))
  (bind (_bblockinghit _binitialoverlap _time _location _impactpoint _normal _impactnormal _physmat _hitactor) (Collision|BreakHitResult Hit))
  (Utilities|FlowControl|Sequence
    (:then_0
      (if (Actor|ActorHasTag _hitactor "Toaster")
        (Game|Damage|ApplyPointDamage 0 (Math|Random|RandomFloatinRange 0.5 1.0) _impactpoint Hit 0 0 "/Game/Blueprints/DamageType_Bullet.DamageType_Bullet_C")
        (Effects|SpawnEmitteratLocation "/Game/Particles/P_Explosion.P_Explosion" _impactpoint)
        (Class|RadialForceComponent|FireImpulse (Variables|Default|GetRadialForce))
        (else
          (Game|Damage|ApplyPointDamage OtherActor (Math|Random|RandomFloatinRange 15.0 25.0) _impactpoint Hit 0 self "/Game/Blueprints/DamageType_Bullet.DamageType_Bullet_C")
          (Effects|SpawnEmitteratLocation "/Game/Particles/P_Explosion.P_Explosion" _impactpoint)
          (Class|RadialForceComponent|FireImpulse (Variables|Default|GetRadialForce))))
      ;[1 1 1] Destroy after a while so that the projectile doesn't go into space and exist forever and ever and ever and ever...
      (Actor|DestroyActor))
    (:then_1
      (switch Utilities|FlowControl|Switch|SwitchonEPhysicalSurface (Variables|/Script/Engine.PhysicalMaterial|GetSurfaceType _physmat) ; Impact Sound
        (:SurfaceType1
          (Audio|PlaySoundatLocation "/Game/Blueprints/Audio/MetalHit_Cue.MetalHit_Cue" _impactpoint "0, 0, 0" (* (Variables|/Game/Blueprints/Viper_GameInstance.Viper_GameInstance_C|GetFXVol (.AsViper%20Game%20Instance (Utilities|Casting|CastToViper_GameInstance (Game|GetGameInstance)))) 1.1)))))))

(event EventBeginPlay
  ;[1 1 1] Destroy after a while so that the projectile doesn't go into space and exist forever and ever and ever and ever...
  (Game|Components|ProjectileMovement|SetVelocityinLocalSpace (Variables|MyProjectile|GetProjectile) (Math|Vector|MakeVector 3e+04 (Math|Random|RandomFloatinRange -5e+01 5e+01) (Math|Random|RandomFloatinRange -5e+01 5e+01))) ; Bullet Spread
  (Utilities|FlowControl|Delay 5.0)
  (Actor|DestroyActor))

(fn ConstructionScript
  (bind _returnvalue (Rendering|Material|CreateDynamicMaterialInstance (Variables|MyProjectile|GetSphere) 0 "/Game/Materials/SpaceBullet_Mat.SpaceBullet_Mat" :!class /Script/Engine.PrimitiveComponent))
  (bind _output_get (Variables|Default|SetBulletInst _returnvalue))
  (Rendering|Material|SetVectorParameterValue _output_get "Color1" "(R=0.478515,G=0.871077,B=0.985000,A=1.000000)" :!class /Script/Engine.MaterialInstanceDynamic)
  (Rendering|Material|SetVectorParameterValue _output_get "Color2" "(R=0.077050,G=0.196714,B=0.670000,A=1.000000)" :!class /Script/Engine.MaterialInstanceDynamic))