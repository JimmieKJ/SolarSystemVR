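; Homing missile for the player's Viper that locks onto the ViperBP's TargetEnemy and explodes with falloff radial damage.
; SelfDestructionCountdown starts the trail and, if tick is enabled, the fire effect, audio, homing and a 20-second fuse.
; Tick eases rotation toward the target and checks a randomized proximity range.
; Fuse expiry, proximity, target loss or collision all feed one DoOnce that applies damage, spawns the explosion and destroys the actor.
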(event OnComponentHit(CollisionComponent)
  (params (OtherActor :type Actor%20Object%20Reference) (OtherComp :type Primitive%20Component%20Object%20Reference) (NormalImpulse :type Vector :default "0, 0, 0") (Hit :type Hit%20Result%20Structure%20%28by%20ref%29))
  (Utilities|FlowControl|DoOnce false
    (:Completed
      (Class|GameplayStatics|ApplyRadialDamagewithFalloff (Variables|Default|GetMaxDamage) 5e+02 (Transformation|GetActorLocation) 5e+02 (Variables|Default|GetDamageRadius) 1.0 "/Game/Blueprints/DamageType_Missile.DamageType_Missile_C" 0 self (Game|GetPlayerController 0) "ECC_Visibility")
      (bind _returnvalue (Effects|SpawnEmitteratLocation "/Game/Particles/P_MissileExplosion.P_MissileExplosion" (Transformation|GetActorLocation)))
      (Class|SceneComponent|DetachfromParent _returnvalue false true)
      (Actor|DestroyActor))))

(event Custom|SelfDestructionCountdown
  (Components|Activation|Activate (Variables|Default|GetMissileTrail) false)
  (if (Class|Actor|IsActorTickEnabled)
    (Components|Activation|Activate (Variables|Default|GetMissileFire) false)
    (Variables|Default|SetTarget (Variables|/Game/Blueprints/ViperBP.ViperBP_C|GetTargetEnemy (.AsViper%20BP (Utilities|Casting|CastToViperBP (Game|Player|GetPlayerPawn 0)))))
    (Variables|/Script/Engine.ProjectileMovementComponent|SetHomingTargetComponent (Variables|MyProjectile|GetProjectile) (Variables|/Game/Blueprints/AIStuff/ToasterBP.ToasterBP_C|GetPlane%20mesh (Variables|Default|GetTarget)))
    (Audio|Components|Audio|Play (Variables|Default|GetAudio) 0.0)
    (Utilities|FlowControl|Delay 2e+01)
    (Utilities|FlowControl|DoOnce false
      (:Completed
        (Class|GameplayStatics|ApplyRadialDamagewithFalloff (Variables|Default|GetMaxDamage) 5e+02 (Transformation|GetActorLocation) 5e+02 (Variables|Default|GetDamageRadius) 1.0 "/Game/Blueprints/DamageType_Missile.DamageType_Missile_C" 0 self (Game|GetPlayerController 0) "ECC_Visibility")
        (bind _returnvalue (Effects|SpawnEmitteratLocation "/Game/Particles/P_MissileExplosion.P_MissileExplosion" (Transformation|GetActorLocation)))
        (Class|SceneComponent|DetachfromParent _returnvalue false true)
        (Actor|DestroyActor)))))

(event EventTick
  (params (DeltaSeconds :type Float%20%28single-precision%29))
  (if (Class|Actor|IsActorTickEnabled)
    (Utilities|IsValid (Variables|Default|GetTarget)
      (:Is%20Valid
        (Utilities|FlowControl|Sequence
          (:then_0
            (if (Math|Float|InRange(Float) (Transformation|GetDistanceTo (Variables|Default|GetTarget)) 0.0 (Math|Random|RandomFloatinRange 3e+02 7.5e+02))
              (Utilities|FlowControl|DoOnce false :!label _label
                (:Completed
                  (Class|GameplayStatics|ApplyRadialDamagewithFalloff (Variables|Default|GetMaxDamage) 5e+02 (Transformation|GetActorLocation) 5e+02 (Variables|Default|GetDamageRadius) 1.0 "/Game/Blueprints/DamageType_Missile.DamageType_Missile_C" 0 self (Game|GetPlayerController 0) "ECC_Visibility")
                  (bind _returnvalue (Effects|SpawnEmitteratLocation "/Game/Particles/P_MissileExplosion.P_MissileExplosion" (Transformation|GetActorLocation)))
                  (Class|SceneComponent|DetachfromParent _returnvalue false true)
                  (Actor|DestroyActor)))))
          (:then_1
            (Transformation|SetActorRotation (Math|Interpolation|RInterpTo (Transformation|GetActorRotation) (Math|Rotator|FindLookatRotation (Transformation|GetActorLocation) (Transformation|GetWorldLocation (Variables|/Game/Blueprints/AIStuff/ToasterBP.ToasterBP_C|GetPlane%20mesh (Variables|Default|GetTarget)))) (Utilities|Time|GetWorldDeltaSeconds) 0.5)))))
      (:Is%20Not%20Valid
        (goto _label)))))

(fn ConstructionScript)