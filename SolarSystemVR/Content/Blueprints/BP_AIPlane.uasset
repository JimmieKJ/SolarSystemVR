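; AI plane actor with three plane meshes that flicker black and white at different rates, apparently as SSVEP visual stimuli.
; Tick runs a separate frame counter per mesh to toggle its Color1 and Color2 material parameters, so flicker frequency depends on frame rate.
; After a random number of flicker cycles, each mesh jumps a random delta-time-scaled distance along its local X axis.
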(event EventTick
  (params (DeltaSeconds :type Float%20%28single-precision%29))
  (Utilities|FlowControl|Sequence
    (:then_0
      (if (< (Variables|Default|GetSSVEPFirstTime) 18)
        (Variables|Default|SetSSVEPFirstTime (+ (Variables|Default|GetSSVEPFirstTime) 1))
        (if (<= (Variables|Default|GetSSVEPFirstTime) 9)
          (Rendering|Material|SetVectorParameterValueonMaterials (Variables|Default|GetPlaneMesh) "Color1" "1.000000,1.000000,1.000000")
          (Rendering|Material|SetVectorParameterValueonMaterials (Variables|Default|GetPlaneMesh) "Color2" "1.000000,1.000000,1.000000")
          (else
            (Rendering|Material|SetVectorParameterValueonMaterials (Variables|Default|GetPlaneMesh) "Color1" "0.000000,0.000000,0.000000")
            (Rendering|Material|SetVectorParameterValueonMaterials (Variables|Default|GetPlaneMesh) "Color2" "0.000000,0.000000,0.000000")))
        (else
          (Variables|Default|SetSSVEPFirstTime 0)
          (bind _output_get (Variables|Default|SetMoveCount (+ (Variables|Default|GetMoveCount) 1)))
          (if (> _output_get (Math|Random|RandomIntegerinRange 10 15))
            (Transformation|AddLocalOffset (Variables|Default|GetPlaneMesh) (* (Math|Vector|MakeVector (Math|Conversions|ToFloat(Integer) (Math|Random|RandomIntegerinRange -10000 10000)) 0.0 0.0) DeltaSeconds) false false)
            (Variables|Default|SetMoveCount 0)))))
    (:then_1
      (if (< (Variables|Default|GetSSVEPSecondTime) 9)
        (Variables|Default|SetSSVEPSecondTime (+ (Variables|Default|GetSSVEPSecondTime) 1))
        (if (<= (Variables|Default|GetSSVEPSecondTime) 5)
          (Rendering|Material|SetVectorParameterValueonMaterials (Variables|Default|GetPlaneMesh1) "Color1" "1.000000,1.000000,1.000000")
          (Rendering|Material|SetVectorParameterValueonMaterials (Variables|Default|GetPlaneMesh1) "Color2" "1.000000,1.000000,1.000000")
          (else
            (Rendering|Material|SetVectorParameterValueonMaterials (Variables|Default|GetPlaneMesh1) "Color1" "0.000000, 0, 0")
            (Rendering|Material|SetVectorParameterValueonMaterials (Variables|Default|GetPlaneMesh1) "Color2" "0.000000, 0, 0")))
        (else
          (Variables|Default|SetSSVEPSecondTime 0)
          (bind _output_get_2 (Variables|Default|SetMoveCount1 (+ (Variables|Default|GetMoveCount1) 1)))
          (if (> _output_get_2 (Math|Random|RandomIntegerinRange 8 13))
            (Transformation|AddLocalOffset (Variables|Default|GetPlaneMesh1) (* (Math|Vector|MakeVector (Math|Conversions|ToFloat(Integer) (Math|Random|RandomIntegerinRange -10000 10000)) 0.0 0.0) DeltaSeconds) false false)
            (Variables|Default|SetMoveCount1 0)))))
    (:then_2
      (if (< (Variables|Default|GetSSVEPThirdTime) 6)
        (Variables|Default|SetSSVEPThirdTime (+ (Variables|Default|GetSSVEPThirdTime) 1))
        (if (<= (Variables|Default|GetSSVEPThirdTime) 3)
          (Rendering|Material|SetVectorParameterValueonMaterials (Variables|Default|GetPlaneMesh2) "Color1" "1.000000,1.000000,1.000000")
          (Rendering|Material|SetVectorParameterValueonMaterials (Variables|Default|GetPlaneMesh2) "Color2" "1.000000,1.000000,1.000000")
          (else
            (Rendering|Material|SetVectorParameterValueonMaterials (Variables|Default|GetPlaneMesh2) "Color1" "0.000000, 0, 0")
            (Rendering|Material|SetVectorParameterValueonMaterials (Variables|Default|GetPlaneMesh2) "Color2" "0.000000, 0, 0")))
        (else
          (Variables|Default|SetSSVEPThirdTime 0)
          (bind _output_get_3 (Variables|Default|SetMoveCount2 (+ (Variables|Default|GetMoveCount2) 1)))
          (if (> _output_get_3 (Math|Random|RandomIntegerinRange 9 14))
            (Transformation|AddLocalOffset (Variables|Default|GetPlaneMesh2) (* (Math|Vector|MakeVector (Math|Conversions|ToFloat(Integer) (Math|Random|RandomIntegerinRange -10000 10000)) 0.0 0.0) DeltaSeconds) false false)
            (Variables|Default|SetMoveCount2 0)))))))

(fn ConstructionScript)