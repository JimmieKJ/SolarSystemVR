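; Landing gear actor for the Viper that extends and retracts its foot linkage and adapts it to the ground below.
; Deploy toggles a ground-check gate and plays or reverses a Timeline that lerps the sledge and strut between stowed and extended positions.
; While the gate is open, Tick traces along the actor's down axis, sets CanLand and clamps foot height to hit distance.
; Look-at rotations, also applied at construction, keep the linked segments aimed at each other.
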(event Custom|Deploy
  (bind _returnvalue (Transformation|GetActorLocation))
  (bind _viperfoot_sledge (Variables|Default|GetViperFoot_Sledge))
  (bind _viperfoot2_2 (Variables|Default|GetViperFoot2_2))
  (bind _relativelocation (Variables|/Script/Engine.SceneComponent|GetRelativeLocation _viperfoot_sledge))
  (bind _relativelocation_2 (Variables|/Script/Engine.SceneComponent|GetRelativeLocation _viperfoot2_2))
  (Utilities|FlowControl|Sequence
    (:then_0
      (Utilities|FlowControl|Gate true) ; enters at Toggle
    )
    (:then_1
      (if (Variables|Default|GetLanding)
        (Variables|Default|SetLanding false)
        (bind _newtrack_0 (Timeline|Timeline_0 Reverse)
          (:Update
            (Transformation|SetRelativeLocation (Variables|Default|GetViperFoot_Sledge) (Math|Vector|Lerp(Vector) "5.000000, 0, 0" (Math|Vector|MakeVector 4.0 0.0 (Math|Float|SelectFloat (* (Math|Float|Clamp(Float) (Variables|Default|GetHitDistance) 0.0 1.6e+02) -1.0) -1.6e+02 (Variables|Default|GetHitTrue))) _newtrack_0) false false)
            (Transformation|SetRelativeLocation (Variables|Default|GetViperFoot2_2) (Math|Vector|Lerp(Vector) "-56.000000, 0,56.000000" (Math|Vector|MakeVector -25.0 0.0 (Math|Float|SelectFloat (* (Math|Float|Clamp(Float) (Variables|Default|GetHitDistance) 0.0 75.0) -1.0) -75.0 (Variables|Default|GetHitTrue))) _newtrack_0) false false)))
        (else
          (Variables|Default|SetLanding true)
          (Timeline|Timeline_0 Play))))))

(event EventTick
  (params (DeltaSeconds :type Float%20%28single-precision%29))
  (bind _returnvalue (Transformation|GetActorLocation))
  (bind _viperfoot_sledge (Variables|Default|GetViperFoot_Sledge))
  (bind _viperfoot2_2 (Variables|Default|GetViperFoot2_2))
  (bind _relativelocation (Variables|/Script/Engine.SceneComponent|GetRelativeLocation _viperfoot_sledge))
  (bind _relativelocation_2 (Variables|/Script/Engine.SceneComponent|GetRelativeLocation _viperfoot2_2))
  (|LookAtRotations)
  (Utilities|FlowControl|Gate true
    (:Exit
      (bind _outhit (Collision|LineTraceByChannel _returnvalue (+ _returnvalue (* (Math|Vector|GetUpVector (Transformation|GetActorRotation)) -7.5e+02)) "TraceTypeQuery1" true 0 "ForOneFrame"))
      (Variables|Default|SetHitTrue (.bblockinghit _outhit))
      (Variables|Default|SetHitDistance (Math|Vector|VectorLength (- _returnvalue (.location _outhit))))
      (Variables|Default|SetCanLand (<= (Math|Vector|VectorLength (- _returnvalue (.location _outhit))) (Variables|Default|GetMaxGroundDistance)))
      (Transformation|SetRelativeLocation _viperfoot_sledge (Math|Vector|MakeVector (.x _relativelocation) (.y _relativelocation) (* (Math|Float|Clamp(Float) (Variables|Default|GetHitDistance) 0.0 1.6e+02) -1.0)) false false)
      (Transformation|SetRelativeLocation _viperfoot2_2 (Math|Vector|MakeVector (.x _relativelocation_2) (.y _relativelocation_2) (* (Math|Float|Clamp(Float) (Variables|Default|GetHitDistance) 0.0 75.0) -1.0)) false false))))

(fn ConstructionScript
  (bind _viperfoot2_2 (Variables|Default|GetViperFoot2_2))
  (bind _viperfoot2_1 (Variables|Default|GetViperFoot2_1))
  (bind _relativelocation (Variables|/Script/Engine.SceneComponent|GetRelativeLocation _viperfoot2_2))
  (Transformation|SetRelativeRotation _viperfoot2_1 (Math|Rotator|FindLookatRotation (Variables|/Script/Engine.SceneComponent|GetRelativeLocation _viperfoot2_1) _relativelocation) false false)
  (Transformation|SetRelativeRotation _viperfoot2_2 (Math|Rotator|FindLookatRotation _relativelocation (Variables|/Script/Engine.SceneComponent|GetRelativeLocation (Variables|Default|GetViperFoot_Sledge))) false false))