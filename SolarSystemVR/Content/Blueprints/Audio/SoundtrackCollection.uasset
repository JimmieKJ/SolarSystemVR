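; Soundtrack actor that plays a configurable music track, scaled by the global music volume.
; The construction script assigns the sound and default volume to its audio component.
; On BeginPlay it waits a set delay, then plays the track at the FlyingGameInstance music volume multiplied by its default volume.
; A SetMusicVolume event lets the volume be rescaled at runtime against that same default.
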(event Custom|SetMusicVolume
  (params (VolumeVar :type Float%20%28single-precision%29))
  (Audio|Components|Audio|SetVolumeMultiplier (Variables|Default|GetAudio) (* VolumeVar (Variables|Default|GetDefaultVol)) :!class /Script/Engine.AudioComponent))

(event EventBeginPlay
  (bind _audio (Variables|Default|GetAudio))
  (Utilities|FlowControl|Delay (Variables|Default|GetDelay))
  (bind _asflying_game_instance (Utilities|Casting|CastToFlyingGameInstance (Game|GetGameInstance)))
  (Audio|Components|Audio|Play _audio 0.0)
  (Audio|Components|Audio|SetVolumeMultiplier _audio (* (Variables|/Game/Blueprints/FlyingGameInstance.FlyingGameInstance_C|GetGlobalMusicVol _asflying_game_instance) (Variables|Default|GetDefaultVol)) :!class /Script/Engine.AudioComponent))

(event EventActorBeginOverlap
  (params (OtherActor :type Actor%20Object%20Reference)))

(event EventTick
  (params (DeltaSeconds :type Float%20%28single-precision%29)))

(fn ConstructionScript
  (bind _audio (Variables|Default|GetAudio))
  (Audio|Components|Audio|SetSound _audio (Variables|Default|GetSound))
  (Audio|Components|Audio|SetVolumeMultiplier _audio (Variables|Default|GetDefaultVol) :!class /Script/Engine.AudioComponent))