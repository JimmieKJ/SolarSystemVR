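; Game instance that holds and persists the game's graphics, audio and best-lap data.
; InitGFX, fired from the main menu, loads saved settings (or saves first-run defaults) and applies them through console commands held in variables.
; Separate events reapply individual options, pushing music volume to SoundtrackCollection actors and FX volume to the player's ViperBP pawn.
; Settings and laps use separate SaveGame classes and slots.
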(event Custom|VSyncActivate
  ;[1 1 1] Set GFX Options
  (Development|ExecuteConsoleCommand (Utilities|String|Append "UseVSync " (Variables|Graphics|GetVSync))))

(event Custom|SetFOV
  ;[1 1 1] Set GFX Options
  (Development|ExecuteConsoleCommand (Utilities|String|Append "fov" " " (Variables|Graphics|GetFOV))))

(event Custom|FullscreenActivate
  ;[1 1 1] Set GFX Options
  (Development|ExecuteConsoleCommand (Variables|Graphics|GetFullscreenSet)))

(event Custom|InitGFX
  ;[1 1 1] Only fires when in Main Menu.
  (CallFunction|SettingsLoad)
  (Development|ExecuteConsoleCommand (Variables|Graphics|GetScreenResolution))
  (Utilities|FlowControl|Sequence
    (:then_0
      (if (Variables|Graphics|GetFullscreenCHECK)
        (Development|ExecuteConsoleCommand (Variables|Graphics|GetFullscreenSet))))
    (:then_1
      (Development|ExecuteConsoleCommand (Utilities|String|Append "fov" " " (Variables|Graphics|GetFOV)))
      (Development|ExecuteConsoleCommand (Utilities|String|Append "GAMMA" " " (Variables|Graphics|GetGamma)))
      (Development|ExecuteConsoleCommand (Utilities|String|Append (Variables|Graphics|GetScreenPercent) " " (Variables|Graphics|GetPercentUI)))
      (CallFunction|MusicVolume (Variables|Audio|GetGlobalMusicVol))
      (CallFunction|FXVolume (Variables|Audio|GetFXVol))
      (Development|ExecuteConsoleCommand (Variables|Graphics|GetPPQuality))
      (Development|ExecuteConsoleCommand (Variables|Graphics|GetShadowQuality))
      (Development|ExecuteConsoleCommand (Variables|Graphics|GetEffectsQuality))
      (Development|ExecuteConsoleCommand (Variables|Graphics|GetAAQuality)))))

(event Custom|FXVolume
  (params (FX :type Float%20%28single-precision%29))
  ;[1 1 1] Set Global VFX Vol. - Fired in OptionsUMG
  (bind _output_get (Variables|Audio|SetFXVol FX))
  (bind _asviper_bp (Utilities|Casting|CastToViperBP (Game|Player|GetPlayerPawn 0)))
  (bind _output_get_2 (Variables|/Game/Blueprints/ViperBP.ViperBP_C|SetFXVolMultiplier _asviper_bp _output_get))
  (Default|FXUpdate _asviper_bp _output_get_2))

(event Custom|MusicVolume
  (params (Music :type Float%20%28single-precision%29))
  ;[1 1 1] Set Global Music Vol. - Fired in OptionsUMG
  (bind _output_get (Variables|Audio|SetGlobalMusicVol Music))
  (bind _outactors (Actor|GetAllActorsOfClass "/Game/Blueprints/Audio/SoundtrackCollection.SoundtrackCollection_C"))
  (for _array_element _outactors
    (Default|SetMusicVolume _array_element _output_get)))

(event Custom|SetGamma
  ;[1 1 1] Set GFX Options
  (Development|ExecuteConsoleCommand (Utilities|String|Append "GAMMA" " " (Variables|Graphics|GetGamma))))

(event Custom|SetGraphics
  (Development|ExecuteConsoleCommand (Variables|Graphics|GetPPQuality))
  (Development|ExecuteConsoleCommand (Variables|Graphics|GetShadowQuality))
  (Development|ExecuteConsoleCommand (Variables|Graphics|GetEffectsQuality))
  (Development|ExecuteConsoleCommand (Variables|Graphics|GetAAQuality)))

(event Custom|ScreenRes
  ;[1 1 1] Set GFX Options
  (Development|ExecuteConsoleCommand (Variables|Graphics|GetScreenResolution)))

(event Custom|SetScreenPercentage
  ;[1 1 1] Set GFX Options
  (Development|ExecuteConsoleCommand (Utilities|String|Append (Variables|Graphics|GetScreenPercent) " " (Variables|Graphics|GetPercentUI))))

(event EventInit)

(fn SettingsSave
  (bind _returnvalue (SaveGame|CreateSaveGameObject "/Game/Blueprints/SaveBPs/Thrusted_GraphicsSave_BP.Thrusted_GraphicsSave_BP_C"))
  (bind _output_get (Variables|SaveSystem|SetSaveGameVar _returnvalue))
  (bind _asthrusted_graphics_save_bp (Utilities|Casting|CastToThrusted_GraphicsSave_BP _output_get))
  (Variables|/Game/Blueprints/SaveBPs/Thrusted_GraphicsSave_BP.Thrusted_GraphicsSave_BP_C|SetMusicVolume _asthrusted_graphics_save_bp (Variables|Audio|GetGlobalMusicVol))
  (Variables|/Game/Blueprints/SaveBPs/Thrusted_GraphicsSave_BP.Thrusted_GraphicsSave_BP_C|SetFXVolume _asthrusted_graphics_save_bp (Variables|Audio|GetFXVol))
  (Variables|/Game/Blueprints/SaveBPs/Thrusted_GraphicsSave_BP.Thrusted_GraphicsSave_BP_C|SetAAQuality _asthrusted_graphics_save_bp (Variables|Graphics|GetAAQuality))
  (Variables|/Game/Blueprints/SaveBPs/Thrusted_GraphicsSave_BP.Thrusted_GraphicsSave_BP_C|SetEffectsQuality _asthrusted_graphics_save_bp (Variables|Graphics|GetEffectsQuality))
  (Variables|/Game/Blueprints/SaveBPs/Thrusted_GraphicsSave_BP.Thrusted_GraphicsSave_BP_C|SetPPQuality _asthrusted_graphics_save_bp (Variables|Graphics|GetPPQuality))
  (Variables|/Game/Blueprints/SaveBPs/Thrusted_GraphicsSave_BP.Thrusted_GraphicsSave_BP_C|SetShadowQuality _asthrusted_graphics_save_bp (Variables|Graphics|GetShadowQuality))
  (Variables|/Game/Blueprints/SaveBPs/Thrusted_GraphicsSave_BP.Thrusted_GraphicsSave_BP_C|SetFOVSave _asthrusted_graphics_save_bp (Variables|Graphics|GetFOV))
  (Variables|/Game/Blueprints/SaveBPs/Thrusted_GraphicsSave_BP.Thrusted_GraphicsSave_BP_C|SetFullscreen _asthrusted_graphics_save_bp (Variables|Graphics|GetFullscreenSet))
  (Variables|/Game/Blueprints/SaveBPs/Thrusted_GraphicsSave_BP.Thrusted_GraphicsSave_BP_C|SetVsync _asthrusted_graphics_save_bp (Variables|Graphics|GetVSync))
  (Variables|/Game/Blueprints/SaveBPs/Thrusted_GraphicsSave_BP.Thrusted_GraphicsSave_BP_C|SetFullscrCheckSave _asthrusted_graphics_save_bp (Variables|Graphics|GetFullscreenCHECK))
  (Variables|/Game/Blueprints/SaveBPs/Thrusted_GraphicsSave_BP.Thrusted_GraphicsSave_BP_C|SetScreenPercentageSave _asthrusted_graphics_save_bp (Variables|Graphics|GetPercentUI))
  (Variables|/Game/Blueprints/SaveBPs/Thrusted_GraphicsSave_BP.Thrusted_GraphicsSave_BP_C|SetScreenRes _asthrusted_graphics_save_bp (Variables|Graphics|GetScreenResolution))
  (Variables|/Game/Blueprints/SaveBPs/Thrusted_GraphicsSave_BP.Thrusted_GraphicsSave_BP_C|SetGammaSave _asthrusted_graphics_save_bp (Variables|Graphics|GetGamma))
  (SaveGame|SaveGametoSlot (Variables|SaveSystem|GetSaveGameVar) (Variables|SaveSystem|GetSettingsSlot)))

(fn SettingsLoad
  (bind _settingsslot (Variables|SaveSystem|GetSettingsSlot))
  (bind _returnvalue (SaveGame|DoesSaveGameExist _settingsslot))
  (if _returnvalue
    (bind _returnvalue_2 (SaveGame|LoadGamefromSlot _settingsslot))
    (bind _asthrusted_graphics_save_bp (Utilities|Casting|CastToThrusted_GraphicsSave_BP _returnvalue_2))
    (Variables|Audio|SetGlobalMusicVol (Variables|/Game/Blueprints/SaveBPs/Thrusted_GraphicsSave_BP.Thrusted_GraphicsSave_BP_C|GetMusicVolume _asthrusted_graphics_save_bp))
    (Variables|Audio|SetFXVol (Variables|/Game/Blueprints/SaveBPs/Thrusted_GraphicsSave_BP.Thrusted_GraphicsSave_BP_C|GetFXVolume _asthrusted_graphics_save_bp))
    (Variables|Graphics|SetShadowQuality (Variables|/Game/Blueprints/SaveBPs/Thrusted_GraphicsSave_BP.Thrusted_GraphicsSave_BP_C|GetShadowQuality _asthrusted_graphics_save_bp))
    (Variables|Graphics|SetEffectsQuality (Variables|/Game/Blueprints/SaveBPs/Thrusted_GraphicsSave_BP.Thrusted_GraphicsSave_BP_C|GetEffectsQuality _asthrusted_graphics_save_bp))
    (Variables|Graphics|SetPercentUI (Variables|/Game/Blueprints/SaveBPs/Thrusted_GraphicsSave_BP.Thrusted_GraphicsSave_BP_C|GetScreenPercentageSave _asthrusted_graphics_save_bp))
    (Variables|Graphics|SetFullscreenSet (Variables|/Game/Blueprints/SaveBPs/Thrusted_GraphicsSave_BP.Thrusted_GraphicsSave_BP_C|GetFullscreen _asthrusted_graphics_save_bp))
    (Variables|Graphics|SetPPQuality (Variables|/Game/Blueprints/SaveBPs/Thrusted_GraphicsSave_BP.Thrusted_GraphicsSave_BP_C|GetPPQuality _asthrusted_graphics_save_bp))
    (Variables|Graphics|SetScreenResolution (Variables|/Game/Blueprints/SaveBPs/Thrusted_GraphicsSave_BP.Thrusted_GraphicsSave_BP_C|GetScreenRes _asthrusted_graphics_save_bp))
    (Variables|Graphics|SetVSync (Variables|/Game/Blueprints/SaveBPs/Thrusted_GraphicsSave_BP.Thrusted_GraphicsSave_BP_C|GetVsync _asthrusted_graphics_save_bp))
    (Variables|Graphics|SetFOV (Variables|/Game/Blueprints/SaveBPs/Thrusted_GraphicsSave_BP.Thrusted_GraphicsSave_BP_C|GetFOVSave _asthrusted_graphics_save_bp))
    (Variables|Graphics|SetAAQuality (Variables|/Game/Blueprints/SaveBPs/Thrusted_GraphicsSave_BP.Thrusted_GraphicsSave_BP_C|GetAAQuality _asthrusted_graphics_save_bp))
    (Variables|Graphics|SetGamma (Variables|/Game/Blueprints/SaveBPs/Thrusted_GraphicsSave_BP.Thrusted_GraphicsSave_BP_C|GetGammaSave _asthrusted_graphics_save_bp))
    (Variables|Graphics|SetFullscreenCHECK (Variables|/Game/Blueprints/SaveBPs/Thrusted_GraphicsSave_BP.Thrusted_GraphicsSave_BP_C|GetFullscrCheckSave _asthrusted_graphics_save_bp))
    (else
      ;[1 1 1] Default screen res. and fullscreen mode when you first run the game.
      (Variables|Graphics|SetFullscreenSet "Nonsense")
      (Variables|Graphics|SetScreenResolution (Utilities|String|Append "r.SetRes " (Utilities|String|Append "1280" "X" "720")))
      (Variables|Graphics|SetFullscreenCHECK false)
      (CallFunction|SettingsSave))))

(fn LapsSave
  (bind _returnvalue (SaveGame|CreateSaveGameObject "/Game/Blueprints/SaveBPs/Thrusted_LapsSave_BP.Thrusted_LapsSave_BP_C"))
  (bind _asthrusted_laps_save_bp (Utilities|Casting|CastToThrusted_LapsSave_BP _returnvalue))
  (Variables|/Game/Blueprints/SaveBPs/Thrusted_LapsSave_BP.Thrusted_LapsSave_BP_C|SetBestLap _asthrusted_laps_save_bp (Variables|Default|GetBestLapSaveVar))
  (Variables|/Game/Blueprints/SaveBPs/Thrusted_LapsSave_BP.Thrusted_LapsSave_BP_C|SetLapTimeTotalSave _asthrusted_laps_save_bp (Variables|Default|GetLapTimeCompare))
  (SaveGame|SaveGametoSlot _asthrusted_laps_save_bp (Variables|SaveSystem|GetLapsSlot)))

(fn LapsLoad
  (bind _returnvalue (SaveGame|DoesSaveGameExist (Variables|SaveSystem|GetLapsSlot)))
  (if _returnvalue
    (bind _returnvalue_2 (SaveGame|LoadGamefromSlot (Variables|SaveSystem|GetLapsSlot)))
    (bind _asthrusted_laps_save_bp (Utilities|Casting|CastToThrusted_LapsSave_BP _returnvalue_2))
    (Variables|Default|SetBestLapSaveVar (Variables|/Game/Blueprints/SaveBPs/Thrusted_LapsSave_BP.Thrusted_LapsSave_BP_C|GetBestLap _asthrusted_laps_save_bp))
    (Variables|Default|SetLapTimeCompare (Variables|/Game/Blueprints/SaveBPs/Thrusted_LapsSave_BP.Thrusted_LapsSave_BP_C|GetLapTimeTotalSave _asthrusted_laps_save_bp))
    (else
      (Variables|Default|SetBestLapSaveVar "-- : -- : --")
      (Variables|Default|SetLapTimeCompare 1e+08))))