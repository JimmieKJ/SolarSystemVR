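; Player controller for the Viper pawn that runs menus, pausing, HUD widgets and mission flow by level name.
; PrecisionTrack times gate runs with a timeline and saves best laps through the GameInstance; other gameplay levels count down reactors.
; Success, death and level opening trigger Viper_CamManager effects, with death also blending to a spawned DeathCam.
; A looping timer rebases the world origin when the pawn strays too far.
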(event Custom|DistanceTracker
  (bind _returnvalue (Game|Player|GetPlayerPawn 0))
  (bind _returnvalue_2 (Transformation|GetActorLocation _returnvalue))
  ;[0.695 0.39 1] Check the distance to world origin and restart or shift origin if too far.
  (if (>= (Math|Vector|VectorLength (Transformation|GetActorLocation _returnvalue)) 2e+06)
    (Class|GameplayStatics|SetWorldOriginLocation (Utilities|Struct|MakeIntVector (Math|Float|Truncate (.x _returnvalue_2)) (Math|Float|Truncate (.y _returnvalue_2)) (Math|Float|Truncate (.z _returnvalue_2))))))

(event Custom|Continue
  ;[1 1 1] Main Menu stuff
  (Variables|Default|SetbShowMouseCursor false)
  (Input|SetInputModeGameandUI 0 0 true true)
  (Variables|Default|SetMenuOpen false)
  (Game|SetGamePaused false)
  (Utilities|IsValid (stale EventBeginPlay _returnvalue_3)
    (:Is%20Valid
      (Widget|RemovefromParent (stale EventBeginPlay _returnvalue_3)))))

(event Custom|ReactorUpdate
  ;[1 0.234 0.1671] Confrontation
  (Variables|/Game/GUI/ReactorCounterUMG.ReactorCounterUMG_C|SetReactorsLeft (stale EventBeginPlay _returnvalue_6) (Utilities|Text|ToText(Integer) (Variables|Default|GetReactorAmount)))
  ;;[1 1 1] Toaster Attack Success
  (if (== (Variables|Default|GetReactorAmount) 0)
    (bind _outactors (Actor|GetAllActorsOfClass "/Game/Blueprints/AIStuff/ToasterBP.ToasterBP_C"))
    (for _array_element _outactors
      _)
    (Utilities|IsValid _array_element
      (:Is%20Not%20Valid
        (Default|MissionComplete (.AsViper%20Cam%20Manager (Utilities|Casting|CastToViper_CamManager (Variables|Default|GetPlayerCameraManager))))))))

(event Custom|IsDead_Event_0
  (bind _returnvalue (Game|Player|GetPlayerPawn 0))
  ;[1 1 1] Death and Death Cam
  (Default|EndGameEffect (.AsViper%20Cam%20Manager (Utilities|Casting|CastToViper_CamManager (Variables|Default|GetPlayerCameraManager))))
  (Utilities|FlowControl|DoOnce false
    (:Completed
      (bind _returnvalue_2 (Game|SpawnActorfromClass "/Game/Blueprints/DeathCam.DeathCam_C" (Math|Transform|MakeTransform (+ (Transformation|GetActorLocation _returnvalue) 1e+02) "0, 0, 0" "1,1,1") "AdjustIfPossibleButAlwaysSpawn" 0 0))
      (Class|Actor|AttachRootComponenttoActor _returnvalue_2 _returnvalue "None" "SnapToTarget" true)
      (Game|Player|SetViewTargetwithBlend _returnvalue_2 1.0 "VTBlend_Linear" 0.0 false))))

(event Custom|FunctionKeyScreen
  (params (TextIn :type Text))
  ;[1 1 1] Warning popups - key(F and G) pressed
  (Utilities|FlowControl|FlipFlop
    (:A
      (Utilities|IsValid (stale _returnvalue_2)
        (:Is%20Valid
          (Widget|RemovefromParent (stale _returnvalue_2)))
        (:Is%20Not%20Valid
          _))
      (bind _output_get (Variables|Default|SetScreenText TextIn))
      (bind _returnvalue (UserInterface|CreateWidget "/Game/GUI/FunctionIndicator_Widget.FunctionIndicator_Widget_C"))
      (Variables|/Game/GUI/FunctionIndicator_Widget.FunctionIndicator_Widget_C|SetHitKey _returnvalue _output_get)
      (UserInterface|Viewport|AddtoViewport _returnvalue 0)
      (Utilities|FlowControl|Delay 2.0)
      (Widget|RemovefromParent _returnvalue))
    (:B
      (Utilities|IsValid _returnvalue
        (:Is%20Valid
          (Widget|RemovefromParent _returnvalue))
        (:Is%20Not%20Valid
          _))
      (bind _output_get_2 (Variables|Default|SetScreenText TextIn))
      (bind _returnvalue_2 (UserInterface|CreateWidget "/Game/GUI/FunctionIndicator_Widget.FunctionIndicator_Widget_C"))
      (Variables|/Game/GUI/FunctionIndicator_Widget.FunctionIndicator_Widget_C|SetHitKey _returnvalue_2 _output_get_2)
      (UserInterface|Viewport|AddtoViewport _returnvalue_2 0)
      (Utilities|FlowControl|Delay 2.0)
      (Widget|RemovefromParent _returnvalue_2))))

(event Custom|Startmatinee_Event_0
  ;[1 0.7525 0.01005] Open Level Matinee.
  (Default|CallMatineeDispatcher)
  (Default|OpenLevel (.AsViper%20Cam%20Manager (Utilities|Casting|CastToViper_CamManager (Variables|Default|GetPlayerCameraManager))))
  (Widget|RemovefromParent (stale EventBeginPlay _returnvalue_3))
  (Variables|Default|SetbShowMouseCursor false))

(event Custom|StartTime
  ;[0.3408 0.685 0.3474] Precision
  (bind _time (Timeline|StartLap PlayFromStart)
    (:Update
      (bind _output_get (Variables|Default|SetLapTime _time))
      (bind _output_get_2 (Variables|Default|SetTimeVar (Utilities|Time _output_get)))
      (bind _output_get_3 (Variables|/Game/GUI/TimerUMG.TimerUMG_C|SetTime (Variables|Default|GetTimerUMG) (Utilities|Text|ToText(String) _output_get_2)))
      (Variables|/Game/GUI/TimerUMG.TimerUMG_C|SetGatesPassed (Variables|Default|GetTimerUMG) (Utilities|Text|ToText(Integer) (Variables|Default|GetGatesPassed)))
      ;;[1 1 1] Gates Success
      (if (== (Variables|Default|GetGatesPassed) (Variables|Default|GetGateAmount))
        (Utilities|FlowControl|DoOnce false :!label _label
          (:Completed
            (CallFunction|StopTime)))
        (else
          (goto _label Reset))))))

(event Custom|StopTime
  (bind _returnvalue (Game|GetGameInstance))
  (bind _asviper_game_instance (Utilities|Casting|CastToViper_GameInstance _returnvalue))
  ;[0.3408 0.685 0.3474] Precision
  (Utilities|FlowControl|Sequence
    (:then_0
      (bind _time (Timeline|StartLap Stop)
        (:Update
          (bind _output_get (Variables|Default|SetLapTime _time))
          (bind _output_get_2 (Variables|Default|SetTimeVar (Utilities|Time _output_get)))
          (bind _output_get_3 (Variables|/Game/GUI/TimerUMG.TimerUMG_C|SetTime (Variables|Default|GetTimerUMG) (Utilities|Text|ToText(String) _output_get_2)))
          (Variables|/Game/GUI/TimerUMG.TimerUMG_C|SetGatesPassed (Variables|Default|GetTimerUMG) (Utilities|Text|ToText(Integer) (Variables|Default|GetGatesPassed)))
          ;;[1 1 1] Gates Success
          (if (== (Variables|Default|GetGatesPassed) (Variables|Default|GetGateAmount))
            (Utilities|FlowControl|DoOnce false :!label _label
              (:Completed
                (CallFunction|StopTime)))
            (else
              (goto _label Reset))))))
    (:then_1
      (Variables|/Game/Blueprints/Viper_GameInstance.Viper_GameInstance_C|SetLapTimeCompare _asviper_game_instance (Math|Float|SelectFloat (Variables|Default|GetLapTime) (Variables|/Game/Blueprints/Viper_GameInstance.Viper_GameInstance_C|GetLapTimeCompare (.AsViper%20Game%20Instance (Utilities|Casting|CastToViper_GameInstance (Game|GetGameInstance)))) (<= (Variables|Default|GetLapTime) (Variables|/Game/Blueprints/Viper_GameInstance.Viper_GameInstance_C|GetLapTimeCompare (.AsViper%20Game%20Instance (Utilities|Casting|CastToViper_GameInstance (Game|GetGameInstance)))))))
      (if (<= (Variables|Default|GetLapTime) (Variables|/Game/Blueprints/Viper_GameInstance.Viper_GameInstance_C|GetLapTimeCompare (.AsViper%20Game%20Instance (Utilities|Casting|CastToViper_GameInstance (Game|GetGameInstance)))))
        (bind _output_get_4 (Variables|/Game/GUI/TimerUMG.TimerUMG_C|SetBestTime (Variables|Default|GetTimerUMG) _output_get_3))
        (Variables|/Game/Blueprints/Viper_GameInstance.Viper_GameInstance_C|SetBestLapSaveVar (.AsViper%20Game%20Instance (Utilities|Casting|CastToViper_GameInstance (Game|GetGameInstance))) _output_get_4))
      (Default|LapsSave _asviper_game_instance)
      (Default|MissionComplete (.AsViper%20Cam%20Manager (Utilities|Casting|CastToViper_CamManager (Variables|Default|GetPlayerCameraManager)))))))

(event EventBeginPlay
  (bind _returnvalue (Game|GetGameInstance))
  (bind _asviper_game_instance (Utilities|Casting|CastToViper_GameInstance _returnvalue))
  ;[1 1 1] Checks which level we are in.
  (bind _returnvalue_2 (Game|GetCurrentLevelName true))
  (if (Utilities|Enum|Equal(Enum) _returnvalue_2 "MainMenu")
    ;[1 1 1] Main Menu stuff
    (bind _returnvalue_3 (UserInterface|CreateWidget "/Game/GUI/MainMenu_UMG.MainMenu_UMG_C"))
    (UserInterface|Viewport|AddtoViewport _returnvalue_3 0)
    (EventDispatchers|AssignStartmatinee (Variables|/Game/GUI/MainMenu_UMG.MainMenu_UMG_C|GetLevelSelect _returnvalue_3) (delegate Custom|Startmatinee_Event_0))
    (Variables|Default|SetbShowMouseCursor true)
    (Input|SetInputModeUIOnly 0 _returnvalue_3 true)
    (Variables|Default|SetMenuOpen true)
    (else
      (Utilities|FlowControl|Sequence
        (:then_0
          (bind _returnvalue_4 (Game|GetCurrentLevelName true))
          (bind _asviper_bp (Utilities|Casting|CastToViperBP (Game|Player|GetPlayerPawn 0)))
          (Variables|Default|SetViper _asviper_bp)
          (if (Utilities|Enum|Equal(Enum) _returnvalue_4 "PrecisionTrack")
            ;[0.3408 0.685 0.3474] Precision
            (Utilities|FlowControl|Sequence
              (:then_0
                (Input|DisableInput (Variables|Default|GetViper) 0)
                (Variables|/Game/Blueprints/ViperBP.ViperBP_C|SetCollisionEndsGame _asviper_bp true)
                (Variables|/Game/Blueprints/ViperBP.ViperBP_C|SetToasterAttack _asviper_bp false))
              (:then_1
                (Utilities|FlowControl|Delay 3.0)
                (Input|EnableInput (Variables|Default|GetViper) 0)
                (bind _returnvalue_5 (UserInterface|CreateWidget "/Game/GUI/TimerUMG.TimerUMG_C"))
                (bind _output_get (Variables|Default|SetTimerUMG _returnvalue_5))
                (UserInterface|Viewport|AddtoViewport _returnvalue_5 0)
                (CallFunction|StartTime)
                (Default|LapsLoad _asviper_game_instance)
                (Variables|/Game/GUI/TimerUMG.TimerUMG_C|SetBestTime (Variables|Default|GetTimerUMG) (Variables|/Game/Blueprints/Viper_GameInstance.Viper_GameInstance_C|GetBestLapSaveVar _asviper_game_instance))))
            (else
              ;[1 0.234 0.1671] Confrontation
              (Variables|/Game/Blueprints/ViperBP.ViperBP_C|SetToasterAttack (Variables|Default|GetViper) true)
              (bind _returnvalue_6 (UserInterface|CreateWidget "/Game/GUI/ReactorCounterUMG.ReactorCounterUMG_C"))
              (UserInterface|Viewport|AddtoViewport _returnvalue_6 0)
              (Variables|/Game/Blueprints/ViperBP.ViperBP_C|SetCollisionEndsGame (Variables|Default|GetViper) true))))
        (:then_1
          ;[0.695 0.39 1] Check the distance to world origin and restart or shift origin if too far.
          (Utilities|Time|SetTimerbyEvent (delegate Custom|DistanceTracker) 15.0 true))))))

(event EventTick
  (params (DeltaSeconds :type Float%20%28single-precision%29))
  (bind _returnvalue (Game|Player|GetPlayerPawn 0))
  (bind _asviper_bp (Utilities|Casting|CastToViperBP _returnvalue))
  ;[1 1 1] Death and Death Cam
  (Utilities|IsValid _asviper_bp
    (:Is%20Valid
      (EventDispatchers|AssignIsDead _asviper_bp (delegate Custom|IsDead_Event_0)))))

(event Input|ActionEvents|InputActionPause
  (params (Key :type Key%20Structure :default "AnyKey"))
  ;[1 1 1] Pause Game
  (:Pressed
    (Utilities|FlowControl|FlipFlop
      (:A
        (Game|SetGamePaused true))
      (:B
        (Game|SetGamePaused false)))))

(event Input|ActionEvents|InputActionMenu
  (params (Key :type Key%20Structure :default "AnyKey"))
  ;[1 1 1] Main Menu stuff
  (:Pressed
    (bind _returnvalue (Game|GetCurrentLevelName true))
    (if (not (Utilities|Enum|Equal(Enum) _returnvalue "MainMenu"))
      (if (Variables|Default|GetMenuOpen)
        (Variables|Default|SetbShowMouseCursor false)
        (Input|SetInputModeGameandUI 0 0 true true)
        (Variables|Default|SetMenuOpen false)
        (Game|SetGamePaused false)
        (Utilities|IsValid (stale _returnvalue_2)
          (:Is%20Valid
            (Widget|RemovefromParent (stale _returnvalue_2))))
        (else
          (Game|SetGamePaused true)
          (bind _returnvalue_2 (UserInterface|CreateWidget "/Game/GUI/MainMenu_UMG.MainMenu_UMG_C"))
          (UserInterface|Viewport|AddtoViewport _returnvalue_2 0)
          (EventDispatchers|AssignStartmatinee (Variables|/Game/GUI/MainMenu_UMG.MainMenu_UMG_C|GetLevelSelect _returnvalue_2) (delegate Custom|Startmatinee_Event_0))
          (Variables|Default|SetbShowMouseCursor true)
          (Input|SetInputModeUIOnly 0 _returnvalue_2 true)
          (Variables|Default|SetMenuOpen true))))))

(fn ConstructionScript)