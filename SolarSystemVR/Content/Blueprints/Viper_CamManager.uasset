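; Viper camera manager that handles screen and audio fades for level start, level transitions, mission completion and player death.
; BeginPlay resets two DoOnce gates and fades in from the fade color.
; Guarded end events fade out: mission completion then flags the Viper game instance's level transition check and opens MainMenu, while death restarts the level by console command.
; OpenLevel only performs a fade-out, without loading a level itself.
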(event Custom|EndGameEffect
  ;[1 1 1] End Game on Death; Fade Out and Restart.
  (Utilities|FlowControl|DoOnce false
    (:Completed
      (CameraFades|StartCameraFade :FromAlpha 0.0 :ToAlpha 1.0 :Duration 7.0 :bShouldFadeAudio true :bHoldWhenFinished true)
      (Utilities|FlowControl|Delay 7.0)
      (Development|ExecuteConsoleCommand "restartlevel"))))

(event Custom|Open%20Level
  (CameraFades|StartCameraFade :FromAlpha 0.0 :ToAlpha 1.0 :Duration 3.5 :bShouldFadeAudio true :bHoldWhenFinished true) ; Open level fade out
)

(event Custom|MissionComplete
  ;[1 1 1] If Mission Complete; Fade Out and Go To Main Menu.
  (Utilities|FlowControl|DoOnce false
    (:Completed
      (Utilities|FlowControl|Delay 3.0)
      (CameraFades|StartCameraFade :FromAlpha 0.0 :ToAlpha 1.0 :Duration 5.0 :bShouldFadeAudio true :bHoldWhenFinished true)
      (Utilities|FlowControl|Delay 5.0)
      (Variables|/Game/Blueprints/Viper_GameInstance.Viper_GameInstance_C|SetLevelTransitionCheck (.AsViper%20Game%20Instance (Utilities|Casting|CastToViper_GameInstance (Game|GetGameInstance))) true) ; Helps tell the game instance whether to fire InitGFX event or not
      (Game|OpenLevel(byName) "MainMenu"))))

(event EventBeginPlay
  (Utilities|FlowControl|Sequence
    (:then_0
      ;[1 1 1] If Mission Complete; Fade Out and Go To Main Menu.
      (Utilities|FlowControl|DoOnce false) ; enters at Reset
    )
    (:then_1
      ;[1 1 1] End Game on Death; Fade Out and Restart.
      (Utilities|FlowControl|DoOnce false) ; enters at Reset
    )
    (:then_2
      (CameraFades|StartCameraFade :FromAlpha 1.0 :ToAlpha 0.0 :Duration 5.0 :bShouldFadeAudio true) ; Game Start Fade In.
    )))

(fn ConstructionScript)