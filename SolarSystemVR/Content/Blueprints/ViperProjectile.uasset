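; ViperProjectile is a fast projectile Blueprint that deals bullet damage and explodes on impact.
; On BeginPlay it launches forward in local space with slight random vertical and lateral spread.
; On hit it applies randomized point damage, spawns an explosion emitter, fires a radial force impulse, then destroys itself.
; A delayed self-destruct removes projectiles that never hit anything.
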(event OnComponentHit(CollisionComponent)
  (params (OtherActor :type Actor%20Object%20Reference) (OtherComp :type Primitive%20Component%20Object%20Reference) (NormalImpulse :type Vector) (Hit :type Hit%20Result%20Structure%20%28by%20ref%29))
  (Game|Damage|ApplyPointDamage OtherActor (Math|Random|RandomFloatinRange 5e+01 75.0) (.ImpactPoint (Collision|BreakHitResult Hit)) Hit 0 0 "/Game/Blueprints/DamageType_Bullet.DamageType_Bullet_C")
  (Effects|SpawnEmitteratLocation "/Game/Particles/P_Explosion.P_Explosion" (Transformation|GetActorLocation))
  (Class|RadialForceComponent|FireImpulse (Variables|Default|GetRadialForce))
  ;[1 1 1] Destroy after a while so that the projectile doesn't go into space and exist forever and ever and ever and ever...
  (Actor|DestroyActor))

(event EventBeginPlay
  ;[1 1 1] Destroy after a while so that the projectile doesn't go into space and exist forever and ever and ever and ever...
  (Game|Components|ProjectileMovement|SetVelocityinLocalSpace (Variables|MyProjectile|GetProjectile) (Math|Vector|MakeVector 4e+04 (Math|Random|RandomFloatinRange -5e+01 5e+01) (Math|Random|RandomFloatinRange -5e+01 5e+01))) ; Bullet Spread
  (Utilities|FlowControl|Delay 5.0)
  (Actor|DestroyActor))

(fn ConstructionScript)