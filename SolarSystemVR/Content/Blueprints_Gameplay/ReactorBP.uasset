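; ReactorBP is a placeable actor that lays out a row of reactors and reports their count to the player.
; Its construction script derives NumofReactors from the horizontal length of the Endpoint vector, then spawns that many child actor components at fixed intervals along local X.
; On BeginPlay it copies the count into the Viper_PlayerController's ReactorAmount and calls ReactorUpdate.
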(event EventBeginPlay
  (bind _asviper_player_controller (Utilities|Casting|CastToViper_PlayerController (Game|GetPlayerController 0)))
  (Variables|/Game/Blueprints/Viper_PlayerController.Viper_PlayerController_C|SetReactorAmount _asviper_player_controller (Variables|Default|GetNumofReactors))
  (Default|ReactorUpdate _asviper_player_controller))

(event EventActorBeginOverlap
  (params (OtherActor :type Actor%20Object%20Reference)))

(event EventTick
  (params (DeltaSeconds :type Float%20%28single-precision%29)))

(fn ConstructionScript
  (bind _endpoint (Variables|Default|GetEndpoint))
  (bind _returnvalue (* _endpoint "1.000000,1.000000, 0"))
  (bind _returnvalue_2 (Math|Vector|VectorLength _returnvalue))
  (bind _returnvalue_3 (/ _returnvalue_2 2.8e+03))
  (bind _returnvalue_4 (Math|Float|Round _returnvalue_3))
  (if (> _returnvalue_4 0)
    (Variables|Default|SetNumofReactors _returnvalue_4)
    (for _index (range 1 _returnvalue_4)
      (bind _returnvalue_5 (AddComponent|AddChildActorComponent false))
      (Transformation|SetRelativeLocation _returnvalue_5 (Math|Vector|MakeVector (* _index 4.2e+03) 0.0 0.0) false false))))